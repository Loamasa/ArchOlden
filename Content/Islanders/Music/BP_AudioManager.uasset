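; Audio manager for Islanders that drives adaptive music in layers, a start-menu score and one-shot transition stingers.
; A Quartz clock starts the Ground, Lift, Conclusion and Focus cues muted and bar-quantized, restoring stored volumes when they begin.
; A bar counter requeues the layers and resets transport every 32 bars, and separately retriggers the menu score.
; Per-layer timelines fade volumes immediately, with Focus fading faster than the others.
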(event `QueueMusic`
  ;[1 1 1] Queue Layer Music
  (bind _returnvalue (`GameplayStatics.CreateSound2D` "/Game/Islanders/Music/S_Ground_Cue.S_Ground_Cue" 1.0 1.0 0.0 null)) ; Core
  (`AudioComponent.SetVolumeMultiplier` _returnvalue 0.0)
  (`AudioComponent.PlayQuantized` _returnvalue (`self.ScoreClock`) (make `QuartzQuantizationBoundary` "Bar" 1.0 "CurrentTimeRelative") (delegate `OnStartGroundLayer`) 0.0 0.0 1.0 "Linear")
  (bind _returnvalue_2 (`GameplayStatics.CreateSound2D` "/Game/Islanders/Music/S_Lift_Cue.S_Lift_Cue" 1.0 1.0 0.0 null)) ; Normal
  (`AudioComponent.SetVolumeMultiplier` _returnvalue_2 0.0)
  (`AudioComponent.PlayQuantized` _returnvalue_2 (`self.ScoreClock`) (make `QuartzQuantizationBoundary` "Bar" 1.0 "CurrentTimeRelative") (delegate `OnStartLiftLayer`) 0.0 0.0 1.0 "Linear")
  (bind _returnvalue_3 (`GameplayStatics.CreateSound2D` "/Game/Islanders/Music/S_Conclusion_Cue.S_Conclusion_Cue" 1.0 1.0 0.0 null)) ; Normal
  (`AudioComponent.SetVolumeMultiplier` _returnvalue_3 0.0)
  (`AudioComponent.PlayQuantized` _returnvalue_3 (`self.ScoreClock`) (make `QuartzQuantizationBoundary` "Bar" 1.0 "CurrentTimeRelative") (delegate `OnStartConclusionLayer`) 0.0 0.0 1.0 "Linear")
  (bind _returnvalue_4 (`GameplayStatics.CreateSound2D` "/Game/Islanders/Music/S_Focus_Cue.S_Focus_Cue" 1.0 1.0 0.0 null)) ; Intensive
  (`AudioComponent.SetVolumeMultiplier` _returnvalue_4 0.0)
  (`AudioComponent.PlayQuantized` _returnvalue_4 (`self.ScoreClock`) (make `QuartzQuantizationBoundary` "Bar" 1.0 "CurrentTimeRelative") (delegate `OnStartFocusLayer`) 0.0 0.0 1.0 "Linear"))

(event `ScoreBarCounter`
  (params (ClockName :type Name) (QuantizationType :type "EQuartzCommandQuantization Enum" :default "Bar") (NumBars :type Integer) (Beat :type Integer) (BeatFraction :type "Float (double-precision)"))
  ;[1 1 1] Count Bars and Retrigger music
  (`self.OnQueueScoreOnBar`)
  (`|ExecutionSequence`
    (:`then_0`
      (if (`self.OnIsScoreMusic`)
        (bind _result (`/Engine/EditorBlueprintResources/StandardMacros.IncrementInt` (`self.CurrentScoreBarCounter`))
          (:`  `
            (if (== _result 32)
              (`self.OnSetScoreMusic` true))))))
    (:`then_1`
      (if (== NumBars 32)
        (`self.QueueMusic`)
        (`QuartzClockHandle.ResetTransportQuantized` :`self` (`self.ScoreClock`) :`InQuantizationBoundary` (make `QuartzQuantizationBoundary` "Bar" 1.0 "CurrentTimeRelative"))))))

(event `OnStartGroundLayer`
  (params (EventType :type "EQuartzCommandDelegateSubType Enum" :default "CommandOnFailedToQueue") (Name :type Name))
  ;[1 1 1] Queue Layer Music
  (switch `EQuartzCommandDelegateSubType` EventType
    (:`CommandOnStarted`
      (bind _output_get (set `self.GroundLayer` (stale `QueueMusic` _returnvalue)))
      (`AudioComponent.SetVolumeMultiplier` _output_get (`self.GroundLayerVolume`)))))

(event `OnStartLiftLayer`
  (params (EventType :type "EQuartzCommandDelegateSubType Enum" :default "CommandOnFailedToQueue") (Name :type Name))
  ;[1 1 1] Queue Layer Music
  (switch `EQuartzCommandDelegateSubType` EventType
    (:`CommandOnStarted`
      (bind _output_get (set `self.LiftLayer` (stale `QueueMusic` _returnvalue_2)))
      (`AudioComponent.SetVolumeMultiplier` _output_get (`self.LiftLayerVolume`)))))

(event `OnStartConclusionLayer`
  (params (EventType :type "EQuartzCommandDelegateSubType Enum" :default "CommandOnFailedToQueue") (Name :type Name))
  ;[1 1 1] Queue Layer Music
  (switch `EQuartzCommandDelegateSubType` EventType
    (:`CommandOnStarted`
      (bind _output_get (set `self.ConclusionLayer` (stale `QueueMusic` _returnvalue_3)))
      (`AudioComponent.SetVolumeMultiplier` _output_get (`self.ConclusionLayerVolume`)))))

(event `OnStartFocusLayer`
  (params (EventType :type "EQuartzCommandDelegateSubType Enum" :default "CommandOnFailedToQueue") (Name :type Name))
  ;[1 1 1] Queue Layer Music
  (switch `EQuartzCommandDelegateSubType` EventType
    (:`CommandOnQueued`
      ;;[1 1 1] Start clock
      (`/Engine/EditorBlueprintResources/StandardMacros.DoOnce` false
        (:`Completed`
          (`QuartzClockHandle.StartClock` (`self.ScoreClock`))
          (`self.ClockStarted`))))
    (:`CommandOnStarted`
      (bind _output_get (set `self.FocusLayer` (stale `QueueMusic` _returnvalue_4)))
      (`AudioComponent.SetVolumeMultiplier` _output_get (`self.FocusLayerVolume`)))))

(event `Instansiate`
  ;[1 1 1] Setup Quartz
  (bind _returnvalue (`QuartzSubsystem.CreateNewClock` (subsystem `QuartzSubsystem`) "ScoreClock" (make `QuartzClockSettings` (make `QuartzTimeSignature` 4)) false true))
  (bind _output_get (set `self.ScoreClock` _returnvalue))
  (bind _clockhandle (`QuartzClockHandle.SetBeatsPerMinute` :`self` _output_get :`BeatsPerMinute` 76.0))
  (`QuartzClockHandle.SubscribeToQuantizationEvent` _clockhandle "Bar" (`|CreateDelegate` :!event `ScoreBarCounter`))
  (`self.QueueMusic`))

(event `OnQueueScore`
  (params (Type :type "/Game/Islanders/Music/E_MusicType Enum" :default "NewEnumerator0"))
  ;[1 1 1] Add music Layers
  (`self.OnSetScoreLayer` true 1.0 Type))

(event `OnSetScoreMusic`
  (params (Activate :type Boolean))
  (if Activate
    (set `self.OnIsScoreMusic` true)
    (bind _returnvalue (`GameplayStatics.CreateSound2D` "/Game/Islanders/Music/S_StartMenu_Cue.S_StartMenu_Cue" 1.0 1.0 0.0 null))
    (bind _output_get (set `self.StartMenuScore` _returnvalue))
    (`AudioComponent.PlayQuantized` _output_get (`self.ScoreClock`) (make `QuartzQuantizationBoundary` "Bar" 1.0 "CurrentTimeRelative") (delegate `OnStartScoreMusic`) 0.0 0.0 1.0 "Linear")
    (else
      (set `self.OnIsScoreMusic` false)
      (goto _label_2 :!via `Open`))))

(event `OnPlayStinger`
  (params (Type :type "/Game/Islanders/Music/E_StingerType Enum" :default "NewEnumerator0"))
  ;[1 1 1] Stingers
  (switch `/Game/Islanders/Music/E_StingerType` Type
    (:`NewEnumerator0`
      (`GameplayStatics.PlaySound2D` "/Game/Islanders/Music/S_EnterFocus_Stinger_Cue.S_EnterFocus_Stinger_Cue" 1.0 1.0 0.0 null null))
    (:`NewEnumerator5`
      (`GameplayStatics.PlaySound2D` "/Game/Islanders/Music/S_ExitFocus_Stinger_Cue.S_ExitFocus_Stinger_Cue" 1.0 1.0 0.0 null null))
    (:`NewEnumerator6`
      (`GameplayStatics.PlaySound2D` "/Game/Islanders/Music/S_Fail_Stringer_Cue.S_Fail_Stringer_Cue" 1.0 1.0 0.0 null null))
    (:`NewEnumerator7`
      (`GameplayStatics.PlaySound2D` "/Game/Islanders/Music/S_Ascended_Stringer_Cue.S_Ascended_Stringer_Cue" 1.0 1.0 0.0 null null))
    (:`NewEnumerator8`
      (`GameplayStatics.PlaySound2D` "/Game/Islanders/Music/S_ToGround_Stringer_Cue.S_ToGround_Stringer_Cue" 1.0 1.0 0.0 null null))
    (:`NewEnumerator9`
      (`GameplayStatics.PlaySound2D` "/Game/Islanders/Music/S_ToLift_Stringer_Cue.S_ToLift_Stringer_Cue" 1.0 1.0 0.0 null null))
    (:`NewEnumerator10`
      (`GameplayStatics.PlaySound2D` "/Game/Islanders/Music/S_ToConclusion_Stringer_Cue.S_ToConclusion_Stringer_Cue" 1.0 1.0 0.0 null null))
    (:`NewEnumerator11`
      (`GameplayStatics.PlaySound2D` "/Game/Islanders/Music/S_ToAscend_Stringer_Cue.S_ToAscend_Stringer_Cue" 1.0 1.0 0.0 null null))))

(event `OnStartScoreMusic`
  (params (EventType :type "EQuartzCommandDelegateSubType Enum" :default "CommandOnFailedToQueue") (Name :type Name))
  (switch `EQuartzCommandDelegateSubType` EventType))

(event `OnQueueScoreOnBar`
  (`|ExecutionSequence`
    (:`then_0`
      (`/Engine/EditorBlueprintResources/StandardMacros.Gate` true :!label _label
        (:`Exit`
          (`|MultiGate` false false 0))))
    (:`then_1`
      (`/Engine/EditorBlueprintResources/StandardMacros.Gate` true :!label _label_2
        (:`Exit`
          (`|ExecutionSequence`
            (:`then_0`
              (goto _label :!via `Open`))
            (:`then_1`
              (`AudioComponent.FadeOut` (`self.StartMenuScore`) 5.066666 0.0 "Logarithmic"))
            (:`then_2`
              (goto _label_2 :!via `Close`))))))))

(event `OnSetScoreLayer`
  (params (Activate :type Boolean) (TargetVolume :type "Float (double-precision)" :default 1.0) (Layer :type "/Game/Islanders/Music/E_MusicType Enum" :default "NewEnumerator0"))
  (bind _normaltimeline (`self.NormalTimeLine`))
  (bind _intimidating (`self.Intimidating`))
  (bind _liftlayer (`self.LiftLayer`))
  (bind _conclusionlayer (`self.ConclusionLayer`))
  (bind _focuslayer (`self.FocusLayer`))
  (bind _intensivetimeline (`self.IntensiveTimeline`))
  (bind _groundlayer (`self.GroundLayer`))
  (bind _calmtimeline (`self.CalmTimeLine`))
  ;[1 1 1] Layer Music
  (set `self.CurrentActivateLayer` Activate)
  (set `self.TargetLayerVolume` TargetVolume)
  (switch `/Game/Islanders/Music/E_MusicType` Layer
    (:`NewEnumerator0`
      ;;[1 1 1] Layer Mixing Immediate with timeline fade
      (if (`self.CurrentActivateLayer`)
        (`TimelineComponent.SetPlayRate` _calmtimeline 0.25)
        (set `self.GroundCurrentVolume` (`self.GroundLayerVolume`))
        (set `self.GroundTargetVolume` (`self.TargetLayerVolume`))
        (bind (_direction _alpha) (`Timeline|CalmTimeLine` :!label _label_3)
          (:`Update`
            (`/Engine/EditorBlueprintResources/StandardMacros.IsValid` _groundlayer
              (:`Is Valid`
                (bind _returnvalue (`KismetMathLibrary.Lerp` (`self.GroundCurrentVolume`) (`self.GroundTargetVolume`) _alpha))
                (`AudioComponent.SetVolumeMultiplier` _groundlayer _returnvalue)
                (set `self.GroundLayerVolume` _returnvalue)))))
        (else
          (`TimelineComponent.SetPlayRate` _calmtimeline 0.25)
          (set `self.GroundCurrentVolume` (`self.TargetLayerVolume`))
          (set `self.GroundTargetVolume` (`self.GroundLayerVolume`))
          (goto _label_3 :!via `ReverseFromEnd`))))
    (:`NewEnumerator1`
      ;;[1 1 1] Layer Mixing Immediate with timeline fade
      (if (`self.CurrentActivateLayer`)
        (`TimelineComponent.SetPlayRate` _normaltimeline 0.25)
        (bind (_direction_2 _alpha_2) (`Timeline|NormalTimeLine` :!label _label_4)
          (:`Update`
            (`/Engine/EditorBlueprintResources/StandardMacros.IsValid` _liftlayer
              (:`Is Valid`
                (bind _returnvalue_2 (`KismetMathLibrary.Lerp` 0.0 (`self.TargetLayerVolume`) _alpha_2))
                (`AudioComponent.SetVolumeMultiplier` _liftlayer _returnvalue_2)
                (set `self.LiftLayerVolume` _returnvalue_2)))))
        (else
          (`TimelineComponent.SetPlayRate` _normaltimeline 0.25)
          (goto _label_4 :!via `ReverseFromEnd`))))
    (:`NewEnumerator2`
      ;;[1 1 1] Layer Mixing Immediate with timeline fade
      (if (`self.CurrentActivateLayer`)
        (`TimelineComponent.SetPlayRate` _intensivetimeline 0.25)
        (bind (_direction_3 _alpha_3) (`Timeline|IntensiveTimeline` :!label _label_5)
          (:`Update`
            (`/Engine/EditorBlueprintResources/StandardMacros.IsValid` _conclusionlayer
              (:`Is Valid`
                (bind _returnvalue_3 (`KismetMathLibrary.Lerp` 0.0 (`self.TargetLayerVolume`) _alpha_3))
                (`AudioComponent.SetVolumeMultiplier` _conclusionlayer _returnvalue_3)
                (set `self.ConclusionLayerVolume` _returnvalue_3)))))
        (else
          (`TimelineComponent.SetPlayRate` _intensivetimeline 0.25)
          (goto _label_5 :!via `ReverseFromEnd`))))
    (:`NewEnumerator3`
      ;;[1 1 1] Layer Mixing Immediate with timeline fade
      (if (`self.CurrentActivateLayer`)
        (`TimelineComponent.SetPlayRate` _intimidating 2.0)
        (bind (_direction_4 _intensivtimeline) (`Timeline|Intimidating` :!label _label_6)
          (:`Update`
            (`/Engine/EditorBlueprintResources/StandardMacros.IsValid` _focuslayer
              (:`Is Valid`
                (bind _returnvalue_4 (`KismetMathLibrary.Lerp` 0.0 (`self.TargetLayerVolume`) _intensivtimeline))
                (`AudioComponent.SetVolumeMultiplier` _focuslayer _returnvalue_4)
                (set `self.FocusLayerVolume` _returnvalue_4)))))
        (else
          (`TimelineComponent.SetPlayRate` _intimidating 0.5)
          (goto _label_6 :!via `ReverseFromEnd`))))))

(fn `PlayCompleteTheme`)

(fn `UserConstructionScript`)