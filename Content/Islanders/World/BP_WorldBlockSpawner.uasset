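; World block spawner that animates one island tile rising into place for BP_WorldGenerator, then bakes it into instanced meshes.
; A timeline raises the preview block after a random delay, then hides it and hands meshes to the Instansiator by block type and decor flag, scattering foliage on non-decor tiles.
; For tiles with resources or artifacts, it has the generator spawn them, then unsubscribes itself.
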(event `Instansiate`
  (`SceneComponent.SetVisibility` (`self.WorldBlock`) false true))

(event `OnPlayEffectAndSpawnMesh`
  (params (Instansiator :type "/Game/Islanders/World/BP_StaticMeshInstantiator Object Reference") (CurrentWorldBlockData :type "MyWorldBlockData Structure") (WorldGenerator :type "/Game/Islanders/World/BP_myWorldGenerator Object Reference") (isDecore :type Boolean :default false) (CurrentSettings :type "/Game/Islanders/StartMenu/S_Settings Structure"))
  (bind _worldblock (`self.WorldBlock`))
  (bind (_relativworldposition_x _relativworldposition_y _relativworldposition_z) (`KismetMathLibrary.BreakVector` (`self.RelativWorldPosition`)))
  (bind ((`CordX` _cordx) (`CordY` _cordy)) (break `MyWorldBlockData` (`self.MyWorldBlockData`)))
  (bind ((`CordX` _cordx_2) (`CordY` _cordy_2) (`Depth` _depth) (`HasArtifactModifier` _hasartifactmodifier) (`HasArtifactAncient` _hasartifactancient) (`HasArtifactWin` _hasartifactwin) (`WorldGenerationArtifacts` _worldgenerationartifacts) (`ModifierArtifacts` _modifierartifacts) (`BuildingArtifacts` _buildingartifacts)) (break `MyWorldBlockData` (`self.MyWorldBlockData`)))
  (bind ((`CordX` _cordx_3) (`CordY` _cordy_3)) (break `MyWorldBlockData` (`self.MyWorldBlockData`)))
  (bind ((`CordX` _cordx_4) (`CordY` _cordy_4)) (break `MyWorldBlockData` (`self.MyWorldBlockData`)))
  (bind ((`CordX` _cordx_5) (`CordY` _cordy_5)) (break `MyWorldBlockData` (`self.MyWorldBlockData`)))
  (bind ((`Depth` _depth_2) (`HasArtifact` _hasartifact) (`WorldGenerationArtifacts` _worldgenerationartifacts_2) (`ModifierArtifacts` _modifierartifacts_2) (`BuildingArtifacts` _buildingartifacts_2) (`NaturalResourcesType` _naturalresourcestype)) (break `MyWorldBlockData` (`self.MyWorldBlockData`)))
  (bind _returnvalue (`SceneComponent.K2_GetComponentLocation` (`self.Box`)))
  (bind _returnvalue_2 (`SceneComponent.K2_GetComponentLocation` (`self.Box`)))
  (bind _returnvalue_3 (`SceneComponent.K2_GetComponentLocation` (`self.Box`)))
  ;[1 1 1] BP_WorldGenerator
  (set `self.Instansiator` Instansiator)
  (set `self.MyWorldBlockData` CurrentWorldBlockData)
  (set `self.WorldGenerator` WorldGenerator)
  (set `self.CurrentIsDecore` isDecore)
  (set `self.Current Settings` CurrentSettings)
  (`KismetArrayLibrary.Array_Clear` (`self.UnusedCorners`))
  (`KismetArrayLibrary.Array_Add` (`self.UnusedCorners`))
  (`KismetArrayLibrary.Array_Add` (`self.UnusedCorners`) 1)
  (`KismetArrayLibrary.Array_Add` (`self.UnusedCorners`) 2)
  (`KismetArrayLibrary.Array_Add` (`self.UnusedCorners`) 3)
  (`SceneComponent.SetRelativeScale3D` (`self.WorldBlock`) (0.2 0.2 0.2))
  (`SceneComponent.K2_SetRelativeLocation` (`self.WorldBlock`) (0.0 0.0 0.0) false false)
  (`SceneComponent.SetVisibility` (`self.WorldBlock`) true true)
  (set `self.StartWaterPosition ` (`KismetMathLibrary.MakeVector` (.x (`SceneComponent.RelativeLocation` (`self.WorldBlock`))) (.y (`SceneComponent.RelativeLocation` (`self.WorldBlock`))) (+ (.z (`SceneComponent.RelativeLocation` (`self.WorldBlock`))) 95.0)))
  (set `self.RelativWorldPosition` (`SceneComponent.RelativeLocation` (`self.WorldBlock`)))
  (`SceneComponent.SetVisibility` (`self.Water`) false false)
  (`SceneComponent.K2_SetRelativeLocation` (`self.Water`) (`self.StartWaterPosition `) false false)
  (switch `MyWorldBlockType` "Grass"
    (:`Grass`
      (`PrimitiveComponent.SetMaterial` _worldblock 0 "/Game/Islanders/World/MI_BasicColor_Grass_Inst.MI_BasicColor_Grass_Inst"))
    (:`Water`
      (`PrimitiveComponent.SetMaterial` _worldblock 0 "/Game/Islanders/World/MI_BasicColor_Water_Inst.MI_BasicColor_Water_Inst")
      (`SceneComponent.SetVisibility` (`self.Water`) true false)
      (`SceneComponent.K2_SetRelativeLocation` (`self.Water`) (`self.StartWaterPosition `) false false))
    (:`Frost`
      (`PrimitiveComponent.SetMaterial` _worldblock 0 "/Game/Islanders/World/MI_BasicColor_Frost_Inst.MI_BasicColor_Frost_Inst"))
    (:`Rock`
      (`PrimitiveComponent.SetMaterial` _worldblock 0 "/Game/Islanders/World/MI_BasicColor_Rock_Inst.MI_BasicColor_Rock_Inst"))
    (:`WBNone`
      (`PrimitiveComponent.SetMaterial` _worldblock 0 "/Game/Islanders/Material/MI_BasicColor_Farm_Inst.MI_BasicColor_Farm_Inst")))
  (bind _output_get (set `self.RelativDepthPosition` (`KismetMathLibrary.MakeVector` _relativworldposition_x _relativworldposition_y (- _relativworldposition_z (`self.StartDepth`)))))
  (`SceneComponent.K2_SetRelativeLocation` (`self.WorldBlock`) _output_get false false)
  (`KismetSystemLibrary.Delay` 0.05)
  (`SceneComponent.SetVisibility` (`self.WorldBlock`) true false)
  (`KismetSystemLibrary.Delay` (`KismetMathLibrary.RandomFloatInRange` 0.0 (`self.TimeForSpawning`)))
  (`|ExecutionSequence`
    (:`then_0`
      (`KismetSystemLibrary.Delay` 0.5)
      (`GameplayStatics.PlaySound2D` "/Game/Islanders/World/S_WorldSpawn_Cue.S_WorldSpawn_Cue" 1.0 1.0 0.0 null null))
    (:`then_1`
      (bind (_direction _alpha) (`Timeline|RaisePillar` :!via `PlayFromStart`)
        (:`Update`
          (`SceneComponent.K2_SetRelativeLocation` (`self.WorldBlock`) (`KismetMathLibrary.VLerp` (`self.RelativDepthPosition`) (`self.RelativWorldPosition`) _alpha) false false))
        (:`Finished`
          (`|ExecutionSequence`
            (:`then_0`
              (if (`self.CurrentIsDecore`)
                (`SceneComponent.SetVisibility` (`self.WorldBlock`) false true)
                (`/Game/Islanders/World/BP_StaticMeshInstantiator.OnAddStaticMeshInstanceSortedByMaterial` (`self.Instansiator`) (`SceneComponent.K2_GetComponentToWorld` (`self.SummitPillar`)) (`StaticMeshComponent.StaticMesh` (`self.SummitPillar`)) "/Game/Islanders/World/M_WorldAlignedColor_Inst.M_WorldAlignedColor_Inst")
                (switch `MyWorldBlockType` (`.WorldBlockType` (break `MyWorldBlockData` (`self.MyWorldBlockData`)))
                  (:`Grass`
                    (`/Game/Islanders/World/BP_StaticMeshInstantiator.OnAddStaticMeshInstanceSortedByMaterial` (`self.Instansiator`) (`SceneComponent.K2_GetComponentToWorld` (`self.WorldBlock`)) (`StaticMeshComponent.StaticMesh` (`self.WorldBlock`)) "/Game/Islanders/World/MI_DecoreMaterial_Grass_Inst.MI_DecoreMaterial_Grass_Inst" :!label _label))
                  (:`Water`
                    (`/Game/Islanders/World/BP_StaticMeshInstantiator.OnAddStaticMeshInstanceSortedByMaterial` (`self.Instansiator`) (`SceneComponent.K2_GetComponentToWorld` (`self.WorldBlock`)) (`StaticMeshComponent.StaticMesh` (`self.WorldBlock`)) "/Game/Islanders/World/MI_WorldMaterial_Water_Inst.MI_WorldMaterial_Water_Inst" :!label _label_2)
                    (`/Game/Islanders/World/BP_StaticMeshInstantiator.OnAddStaticMeshInstanceSortedByMaterial` (`self.Instansiator`) (`SceneComponent.K2_GetComponentToWorld` (`self.Water`)) (`StaticMeshComponent.StaticMesh` (`self.Water`)) "/Game/Islanders/World/MI_water_Inst.MI_water_Inst"))
                  (:`Frost`
                    (`/Game/Islanders/World/BP_StaticMeshInstantiator.OnAddStaticMeshInstanceSortedByMaterial` (`self.Instansiator`) (`SceneComponent.K2_GetComponentToWorld` (`self.WorldBlock`)) (`StaticMeshComponent.StaticMesh` (`self.WorldBlock`)) "/Game/Islanders/World/MI_WorldMaterial_Frost_Inst.MI_WorldMaterial_Frost_Inst"))
                  (:`Rock`
                    (`/Game/Islanders/World/BP_StaticMeshInstantiator.OnAddStaticMeshInstanceSortedByMaterial` (`self.Instansiator`) (`SceneComponent.K2_GetComponentToWorld` (`self.WorldBlock`)) (`StaticMeshComponent.StaticMesh` (`self.WorldBlock`)) "/Game/Islanders/World/MI_DecoreMaterial_Rock_Inst.MI_DecoreMaterial_Rock_Inst"))
                  (:`WBNone`
                    (`/Engine/EditorBlueprintResources/StandardMacros.FlipFlop`
                      (:`A`
                        (goto _label))
                      (:`B`
                        (goto _label_2)))))
                (else
                  (`SceneComponent.SetVisibility` (`self.WorldBlock`) false true)
                  (`/Game/Islanders/World/BP_StaticMeshInstantiator.OnAddStaticMeshInstanceSortedByMaterial` (`self.Instansiator`) (`SceneComponent.K2_GetComponentToWorld` (`self.SummitPillar`)) (`StaticMeshComponent.StaticMesh` (`self.SummitPillar`)) "/Game/Islanders/World/M_WorldAlignedColor_Inst.M_WorldAlignedColor_Inst")
                  (switch `MyWorldBlockType` (`.WorldBlockType` (break `MyWorldBlockData` (`self.MyWorldBlockData`)))
                    (:`Grass`
                      (`/Game/Islanders/World/BP_StaticMeshInstantiator.OnAddStaticMeshInstanceSortedByMaterial` (`self.Instansiator`) (`SceneComponent.K2_GetComponentToWorld` (`self.WorldBlock`)) (`StaticMeshComponent.StaticMesh` (`self.WorldBlock`)) "/Game/Islanders/World/MI_WorldMaterial_Grass_Inst.MI_WorldMaterial_Grass_Inst" :!label _label_3)
                      (if (and (< 0.2 (`KismetMathLibrary.RandomFloatInRange` 0.0 1.0)) (`.HasNaturalResoruces` (break `MyWorldBlockData` (`self.MyWorldBlockData`))))
                        (`/Game/Islanders/World/BP_StaticMeshInstantiator.OnAddStaticMeshInstanceSortedByMesh` (`self.Instansiator`) (`KismetMathLibrary.MakeTransform` (`KismetMathLibrary.MakeVector` (.x (`KismetMathLibrary.RandomPointInBoundingBox` _returnvalue (* (`BoxComponent.BoxExtent` (`self.Box`)) 0.2))) (.y (`KismetMathLibrary.RandomPointInBoundingBox` _returnvalue (* (`BoxComponent.BoxExtent` (`self.Box`)) 0.2))) (.z _returnvalue)) (`KismetMathLibrary.MakeRotator` 0.0 0.0 (`KismetMathLibrary.RandomFloatInRange` 0.0 360.0)) (`KismetMathLibrary.MakeVector` (`KismetMathLibrary.RandomFloatInRange` 0.6 1.0) (`KismetMathLibrary.RandomFloatInRange` 0.6 1.0) 1.0)) (`|GetArrayItem` (`|MakeArray` "/Game/Islanders/World/FoliageFlat/SM_Foliage_Grass_1.SM_Foliage_Grass_1" "/Game/Islanders/World/FoliageFlat/SM_Foliage_Grass_2.SM_Foliage_Grass_2" "/Game/Islanders/World/FoliageFlat/SM_Foliage_Grass_3.SM_Foliage_Grass_3" "/Game/Islanders/World/FoliageFlat/SM_Foliage_Grass_4.SM_Foliage_Grass_4" "/Game/Islanders/World/FoliageFlat/SM_Foliage_Grass_5.SM_Foliage_Grass_5" "/Game/Islanders/World/FoliageFlat/SM_Foliage_Grass_6.SM_Foliage_Grass_6" "/Game/Islanders/World/FoliageFlat/SM_Foliage_Grass_7.SM_Foliage_Grass_7" "/Game/Islanders/World/FoliageFlat/SM_Foliage_Grass_8.SM_Foliage_Grass_8" :!type "StaticMesh Object Reference") (`KismetMathLibrary.RandomIntegerInRange` 0 7)))))
                    (:`Water`
                      (`/Game/Islanders/World/BP_StaticMeshInstantiator.OnAddStaticMeshInstanceSortedByMaterial` (`self.Instansiator`) (`SceneComponent.K2_GetComponentToWorld` (`self.WorldBlock`)) (`StaticMeshComponent.StaticMesh` (`self.WorldBlock`)) "/Game/Islanders/World/MI_WorldMaterial_Water_Inst.MI_WorldMaterial_Water_Inst" :!label _label_4)
                      (`/Game/Islanders/World/BP_StaticMeshInstantiator.OnAddStaticMeshInstanceSortedByMaterial` (`self.Instansiator`) (`SceneComponent.K2_GetComponentToWorld` (`self.Water`)) (`StaticMeshComponent.StaticMesh` (`self.Water`)) "/Game/Islanders/World/MI_water_Inst.MI_water_Inst"))
                    (:`Frost`
                      (`/Game/Islanders/World/BP_StaticMeshInstantiator.OnAddStaticMeshInstanceSortedByMaterial` (`self.Instansiator`) (`SceneComponent.K2_GetComponentToWorld` (`self.WorldBlock`)) (`StaticMeshComponent.StaticMesh` (`self.WorldBlock`)) "/Game/Islanders/World/MI_WorldMaterial_Frost_Inst.MI_WorldMaterial_Frost_Inst")
                      (if (`.isSpawningParticles_11_BEDBAEE1438AE952358C368D2E53A1AC` (break `/Game/Islanders/StartMenu/S_Settings` (`self.Current Settings`)))
                        (`GameplayStatics.SpawnEmitterAtLocation` "/Game/Islanders/Particles/P_Snow.P_Snow" (`SceneComponent.K2_GetComponentLocation` (`self.DefaultSceneRoot`))))
                      (if (< 0.6 (`KismetMathLibrary.RandomFloatInRange` 0.0 1.0))
                        (`/Game/Islanders/World/BP_StaticMeshInstantiator.OnAddStaticMeshInstanceSortedByMesh` (`self.Instansiator`) (`KismetMathLibrary.MakeTransform` (`KismetMathLibrary.MakeVector` (.x (`KismetMathLibrary.RandomPointInBoundingBox` _returnvalue_2 (* (`BoxComponent.BoxExtent` (`self.Box`)) 0.2))) (.y (`KismetMathLibrary.RandomPointInBoundingBox` _returnvalue_2 (* (`BoxComponent.BoxExtent` (`self.Box`)) 0.2))) (.z _returnvalue_2)) (`KismetMathLibrary.MakeRotator` 0.0 0.0 (`KismetMathLibrary.RandomFloatInRange` 0.0 360.0)) (`KismetMathLibrary.MakeVector` (`KismetMathLibrary.RandomFloatInRange` 0.6 1.0) (`KismetMathLibrary.RandomFloatInRange` 0.6 1.0) 1.0)) (`|GetArrayItem` (`|MakeArray` "/Game/Islanders/World/FoliageFlat/SM_Foliage_Snow_1.SM_Foliage_Snow_1" "/Game/Islanders/World/FoliageFlat/SM_Foliage_Snow_2.SM_Foliage_Snow_2" "/Game/Islanders/World/FoliageFlat/SM_Foliage_Snow_3.SM_Foliage_Snow_3" "/Game/Islanders/World/FoliageFlat/SM_Foliage_Snow_4.SM_Foliage_Snow_4" :!type "StaticMesh Object Reference") (`KismetMathLibrary.RandomIntegerInRange` 0 3)))))
                    (:`Rock`
                      (`/Game/Islanders/World/BP_StaticMeshInstantiator.OnAddStaticMeshInstanceSortedByMaterial` (`self.Instansiator`) (`SceneComponent.K2_GetComponentToWorld` (`self.WorldBlock`)) (`StaticMeshComponent.StaticMesh` (`self.WorldBlock`)) "/Game/Islanders/World/MI_WorldMaterial_Rock_InstN.MI_WorldMaterial_Rock_InstN")
                      (if (< 0.7 (`KismetMathLibrary.RandomFloatInRange` 0.0 1.0))
                        (`/Game/Islanders/World/BP_StaticMeshInstantiator.OnAddStaticMeshInstanceSortedByMesh` (`self.Instansiator`) (`KismetMathLibrary.MakeTransform` (`KismetMathLibrary.MakeVector` (.x (`KismetMathLibrary.RandomPointInBoundingBox` _returnvalue_3 (* (`BoxComponent.BoxExtent` (`self.Box`)) 0.2))) (.y (`KismetMathLibrary.RandomPointInBoundingBox` _returnvalue_3 (* (`BoxComponent.BoxExtent` (`self.Box`)) 0.2))) (.z _returnvalue_3)) (`KismetMathLibrary.MakeRotator` 0.0 0.0 (`KismetMathLibrary.RandomFloatInRange` 0.0 360.0)) (`KismetMathLibrary.MakeVector` (`KismetMathLibrary.RandomFloatInRange` 0.6 1.0) (`KismetMathLibrary.RandomFloatInRange` 0.6 1.0) 1.0)) (`|GetArrayItem` (`|MakeArray` "/Game/Islanders/World/FoliageFlat/SM_Foliage_Rock_1.SM_Foliage_Rock_1" "/Game/Islanders/World/FoliageFlat/SM_Foliage_Rock_2.SM_Foliage_Rock_2" "/Game/Islanders/World/FoliageFlat/SM_Foliage_Rock_3.SM_Foliage_Rock_3" "/Game/Islanders/World/FoliageFlat/SM_Foliage_Rock_4.SM_Foliage_Rock_4" :!type "StaticMesh Object Reference") (`KismetMathLibrary.RandomIntegerInRange` 0 3)))))
                    (:`WBNone`
                      (`/Engine/EditorBlueprintResources/StandardMacros.FlipFlop`
                        (:`A`
                          (goto _label_3))
                        (:`B`
                          (goto _label_4))))))))
            (:`then_1`
              (if (or (`|EnumInequality` _naturalresourcestype "NR_None") _hasartifact)
                (`KismetSystemLibrary.Delay` (`KismetMathLibrary.RandomFloatInRange` 0.05 0.2))
                (`|ExecutionSequence`
                  (:`then_0`
                    (switch `MyNaturalResourcesType` (`.NaturalResourcesType` (break `MyWorldBlockData` (`self.MyWorldBlockData`)))
                      (:`NR_Tree`
                        (for _ (`.NaturalResources` (break `MyWorldBlockData` (`self.MyWorldBlockData`)))
                          (set `self.TempIndex` (`KismetMathLibrary.RandomIntegerInRange` 0 (- (`KismetArrayLibrary.Array_Length` (`self.UnusedCorners`)) 1)))
                          (switch `int` (`|GetArrayItem` (`self.UnusedCorners`) (`self.TempIndex`))
                            (:`Default`
                              (`KismetSystemLibrary.PrintString` "plipp"))
                            (:`0`
                              (set `self.CurrentCorner` "UpperRight")
                              (`/Game/Islanders/World/BP_myWorldGenerator.SpawnEnviormentOnWorldBlock` (`self.WorldGenerator`) "Tree" (`self.K2_GetActorLocation`) (`self.CurrentCorner`) "OneBlock" :!label _label_5)
                              (`KismetArrayLibrary.Array_Remove` (`self.UnusedCorners`) (`self.TempIndex`)))
                            (:`1`
                              (set `self.CurrentCorner` "UpperLeft")
                              (goto _label_5))
                            (:`2`
                              (set `self.CurrentCorner` "BelowRight")
                              (goto _label_5))
                            (:`3`
                              (set `self.CurrentCorner` "BelowLeft")
                              (goto _label_5)))))
                      (:`NR_Fish`
                        (for (_ _array_index) (`.NaturalResources` (break `MyWorldBlockData` (`self.MyWorldBlockData`)))
                          (`/Game/Islanders/World/BP_myWorldGenerator.SpawnEnviormentOnWorldBlock` (`self.WorldGenerator`) "Fish" (`self.K2_GetActorLocation`) (cast `MyCorner` (`KismetMathLibrary.Conv_IntToByte` _array_index)) "OneBlock")))
                      (:`NR_Mineral`
                        (for _ (`.NaturalResources` (break `MyWorldBlockData` (`self.MyWorldBlockData`)))
                          (set `self.TempIndex` (`KismetMathLibrary.RandomIntegerInRange` 0 (- (`KismetArrayLibrary.Array_Length` (`self.UnusedCorners`)) 1)))
                          (`/Game/Islanders/World/BP_myWorldGenerator.SpawnEnviormentOnWorldBlock` (`self.WorldGenerator`) "Mineral" (`self.K2_GetActorLocation`) (cast `MyCorner` (`KismetMathLibrary.Conv_IntToByte` (`|GetArrayItem` (`self.UnusedCorners`) (`self.TempIndex`)))) "OneBlock")
                          (`KismetArrayLibrary.Array_Remove` (`self.UnusedCorners`) (`self.TempIndex`))))
                      (:`NR_Crystal`
                        (for (_ _array_index_2) (`.NaturalResources` (break `MyWorldBlockData` (`self.MyWorldBlockData`)))
                          (`/Game/Islanders/World/BP_myWorldGenerator.SpawnEnviormentOnWorldBlock` (`self.WorldGenerator`) "Crystal" (`self.K2_GetActorLocation`) (cast `MyCorner` (`KismetMathLibrary.Conv_IntToByte` _array_index_2)) "FourBlock")))))
                  (:`then_1`
                    (if (`.HasArtifact` (break `MyWorldBlockData` (`self.MyWorldBlockData`)))
                      (`|ExecutionSequence`
                        (:`then_0`
                          (if (`|EnumInequality` _worldgenerationartifacts "AGT_None")
                            (`/Game/Islanders/World/BP_myWorldGenerator.SpawnArtifactOnBlock` (`self.WorldGenerator`) _cordx_3 _cordy_3 false false false _worldgenerationartifacts "None" (`self.K2_GetActorLocation`))))
                        (:`then_1`
                          (if _modifierartifacts
                            (`/Game/Islanders/World/BP_myWorldGenerator.SpawnArtifactOnBlock` (`self.WorldGenerator`) _cordx_4 _cordy_4 true false false "AGT_None" "None" (`self.K2_GetActorLocation`))))
                        (:`then_2`
                          (if (`|EnumInequality` _buildingartifacts)
                            (`/Game/Islanders/World/BP_myWorldGenerator.SpawnArtifactOnBlock` (`self.WorldGenerator`) _cordx_5 _cordy_5 false false false "AGT_None" _buildingartifacts (`self.K2_GetActorLocation`))))
                        (:`then_3`
                          (if _hasartifactwin
                            (`/Game/Islanders/World/BP_myWorldGenerator.SpawnArtifactOnBlock` (`self.WorldGenerator`) _cordx _cordy false false true "AGT_None" "None" (`self.K2_GetActorLocation`)))))))
                  (:`then_2`
                    (`/Game/Islanders/World/BP_myWorldGenerator.UnSubscribeWorldBlockEffect` (`self.WorldGenerator`) self)))))))))))

(fn `AssigneNaturalresources`
  (params (WorldBlockData :type "MyWorldBlockData Structure") (BuildingTypes :type "MyBuildingType Enum" :default "Tree"))
  (locals (TempBuildingType :type "MyBuildingType Enum") (TempWorldBlockData :type " Structure") (TempMyWorldBlockData :type "MyWorldBlockData Structure"))
  (set `local.TempMyWorldBlockData` WorldBlockData)
  (set `local.TempBuildingType` BuildingTypes)
  (for _ (`.NaturalResources` (break `MyWorldBlockData` (`local.TempMyWorldBlockData`)))
    (set `self.TempIndex` (`KismetMathLibrary.RandomIntegerInRange` 0 (- (`KismetArrayLibrary.Array_Length` (`self.UnusedCorners`)) 1)))
    (if (`.HasNaturalResoruces` (break `MyWorldBlockData` (`local.TempMyWorldBlockData`)))
      (`/Game/Islanders/World/BP_myWorldGenerator.SpawnEnviormentOnWorldBlock` (`self.WorldGenerator`) (`local.TempBuildingType`) (`self.K2_GetActorLocation`) (cast `MyCorner` (`KismetMathLibrary.Conv_IntToByte` (`|GetArrayItem` (`self.UnusedCorners`) (`self.TempIndex`)))) "OneBlock")
      (`KismetArrayLibrary.Array_Remove` (`self.UnusedCorners`) (`self.TempIndex`)))))

(fn `UserConstructionScript`)