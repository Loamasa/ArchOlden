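; BP_WorldBlock is a single grid block of the Islanders world, storing its coordinates, type and decorated state.
; Setting its type swaps material, tags the collision box and adjusts water, then raises the block from below via a timeline with randomly staggered delay and sound.
; Box overlaps return neighboring blocks or their types.
; A cleanup event hides its individual meshes once they are converted to static mesh instances.
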(event `OnSetActive`
  (params (IsActive :type Boolean))
  (`SceneComponent.SetVisibility` (`self.WorldBlock`) IsActive false))

(event `OnCleanUpAfterStaticMeshInstanciation`
  (bind _worldblock (`self.WorldBlock`))
  (bind _water (`self.Water`))
  (bind _summitpillar (`self.SummitPillar`))
  (set `self.IsMeshInstanciated` true)
  (`|ExecutionSequence`
    (:`then_0`
      (`/Engine/EditorBlueprintResources/StandardMacros.IsValid` _summitpillar
        (:`Is Valid`
          (`SceneComponent.SetVisibility` _summitpillar false false))))
    (:`then_1`
      (`/Engine/EditorBlueprintResources/StandardMacros.IsValid` _water
        (:`Is Valid`
          (`SceneComponent.SetVisibility` _water false false))))
    (:`then_2`
      (`/Engine/EditorBlueprintResources/StandardMacros.IsValid` _worldblock
        (:`Is Valid`
          (`SceneComponent.SetVisibility` _worldblock false false))))))

(event `Instansitate`
  (params (Xposition :type Integer) (YPosition :type Integer) (WorldBlockType :type "/Game/Islanders/World/E_WorldBlockType Enum" :default "NewEnumerator0") (RelativeScale :type "Vector Structure") (SpawnEffectTime :type "Float (double-precision)"))
  (bind _returnvalue_location (`KismetMathLibrary.BreakTransform` (`SceneComponent.GetRelativeTransform` (`self.Water`))))
  (set `self.XPosition` Xposition)
  (set `self.YPosition` YPosition)
  (set `self.BlockType` WorldBlockType)
  (`SceneComponent.SetRelativeScale3D` (`self.WorldBlock`) RelativeScale)
  (set `self.TimeForSpawning` SpawnEffectTime)
  (set `self.StartWaterPosition ` _returnvalue_location)
  (set `self.RelativWorldPosition` (`SceneComponent.RelativeLocation` (`self.WorldBlock`)))
  (`self.OnSetNewWorldType` (`self.BlockType`)))

(event `OnSetNewWorldType`
  (params (WorldBlockType :type "/Game/Islanders/World/E_WorldBlockType Enum" :default "NewEnumerator0"))
  (bind _worldblock (`self.WorldBlock`))
  (bind (_relativworldposition_x _relativworldposition_y _relativworldposition_z) (`KismetMathLibrary.BreakVector` (`self.RelativWorldPosition`)))
  ;[1 1 1] BP_WorldGenerator
  (set `self.BlockType` WorldBlockType)
  (set `ActorComponent.ComponentTags` (`|MakeArray` (`KismetStringLibrary.Conv_StringToName` (`|GetEnumeratorNameAsString` (`self.BlockType`)))) (`self.CollisionBox`))
  (`SceneComponent.SetVisibility` (`self.Water`) false false)
  (`SceneComponent.K2_SetRelativeLocation` (`self.Water`) (`self.StartWaterPosition `) false false)
  (switch `/Game/Islanders/World/E_WorldBlockType` (`self.BlockType`)
    (:`NewEnumerator0`
      (`PrimitiveComponent.SetMaterial` _worldblock 0 "/Game/Islanders/World/MI_BasicColor_Grass_Inst.MI_BasicColor_Grass_Inst"))
    (:`NewEnumerator1`
      (`PrimitiveComponent.SetMaterial` _worldblock 0 "/Game/Islanders/World/MI_BasicColor_Water_Inst.MI_BasicColor_Water_Inst")
      (`SceneComponent.SetVisibility` (`self.Water`) true false)
      (`SceneComponent.K2_SetRelativeLocation` (`self.Water`) (`KismetMathLibrary.MakeVector` (.x (`self.StartWaterPosition `)) (.y (`self.StartWaterPosition `)) (+ (.z (`self.StartWaterPosition `)) 50.0)) false false)
      (`SceneComponent.K2_SetRelativeLocation` (`self.CollisionBox`) (`KismetMathLibrary.MakeVector` (.x (`self.StartWaterPosition `)) (.y (`self.StartWaterPosition `)) (+ (.z (`self.StartWaterPosition `)) 25.0)) false false))
    (:`NewEnumerator3`
      (`PrimitiveComponent.SetMaterial` _worldblock 0 "/Game/Islanders/World/MI_BasicColor_Frost_Inst.MI_BasicColor_Frost_Inst"))
    (:`NewEnumerator2`
      (`PrimitiveComponent.SetMaterial` _worldblock 0 "/Game/Islanders/World/MI_BasicColor_Rock_Inst.MI_BasicColor_Rock_Inst"))
    (:`NewEnumerator4`
      (`PrimitiveComponent.SetMaterial` _worldblock 0 "/Game/Islanders/Material/MI_BasicColor_Farm_Inst.MI_BasicColor_Farm_Inst")))
  (bind _output_get (set `self.RelativDepthPosition` (`KismetMathLibrary.MakeVector` _relativworldposition_x _relativworldposition_y (- _relativworldposition_z (`self.StartDepth`)))))
  (`SceneComponent.K2_SetRelativeLocation` (`self.WorldBlock`) _output_get false false)
  (`KismetSystemLibrary.Delay` 0.05)
  (`SceneComponent.SetVisibility` (`self.WorldBlock`) true false)
  (`KismetSystemLibrary.Delay` (`KismetMathLibrary.RandomFloatInRange` 0.0 (`self.TimeForSpawning`)))
  (`|ExecutionSequence`
    (:`then_0`
      (`KismetSystemLibrary.Delay` 0.5)
      (`GameplayStatics.PlaySound2D` "/Game/Islanders/World/S_WorldSpawn_Cue.S_WorldSpawn_Cue" 1.0 1.0 0.0 null null))
    (:`then_1`
      (bind (_direction _alpha) (`Timeline|RaisePillar`)
        (:`Update`
          (`SceneComponent.K2_SetRelativeLocation` (`self.WorldBlock`) (`KismetMathLibrary.VLerp` (`self.RelativDepthPosition`) (`self.RelativWorldPosition`) _alpha) false false)
          (`self.IsSpawned`))))))

(fn `GetWorldBlockType`
  (returns (WorldBlockType :type "/Game/Islanders/World/E_WorldBlockType Enum"))
  (return (`self.BlockType`)))

(fn `GetXandY`
  (returns (X :type Integer) (Y :type Integer))
  (return (`self.XPosition`) (`self.YPosition`)))

(fn `On Get Surrounding Block Types`
  (returns (SurroundingBlockTypes :type "Array of /Game/Islanders/World/E_WorldBlockType Enum"))
  (locals (SurroundingBlockTypesTemp :type "Array of /Game/Islanders/World/E_WorldBlockType Enum"))
  (`KismetArrayLibrary.Array_Clear` (`local.SurroundingBlockTypesTemp`))
  (bind _outactors (`KismetSystemLibrary.BoxOverlapActors` (`SceneComponent.K2_GetComponentLocation` (`self.WorldBlock`)) (15.0 15.0 3.0) (`|MakeArray` "ObjectTypeQuery8" :!type "EObjectTypeQuery Enum") "BP_WorldBlock_C"))
  (for _array_element _outactors
    (bind _asbp_world_block (cast `/Game/Islanders/World/BP_WorldBlock` _array_element))
    (bind _worldblocktype (`self.GetWorldBlockType` _asbp_world_block))
    (`KismetArrayLibrary.Array_Add` (`local.SurroundingBlockTypesTemp`) _worldblocktype)
    ;[1 1 1] Remove this blocks type
    (if (`|EnumEquality` _worldblocktype (`self.BlockType`))
      (`/Engine/EditorBlueprintResources/StandardMacros.DoOnce` false
        (:`Completed`
          (`KismetArrayLibrary.Array_RemoveItem` (`local.SurroundingBlockTypesTemp`) (`self.BlockType`))))))
  (return (`local.SurroundingBlockTypesTemp`)))

(fn `On Get SurroundingBlocks`
  (returns (SurroundingBlockTypes :type "Array of /Game/Islanders/World/BP_WorldBlock Object Reference"))
  (locals (SurroundingBlockTypesTemp :type "Array of /Game/Islanders/World/BP_WorldBlock Object Reference"))
  (`KismetArrayLibrary.Array_Clear` (`local.SurroundingBlockTypesTemp`))
  (bind _outactors (`KismetSystemLibrary.BoxOverlapActors` (`SceneComponent.K2_GetComponentLocation` (`self.WorldBlock`)) (15.0 15.0 5.0) (`|MakeArray` "ObjectTypeQuery8" :!type "EObjectTypeQuery Enum") "BP_WorldBlock_C"))
  (for _array_element _outactors
    (bind _asbp_world_block (cast `/Game/Islanders/World/BP_WorldBlock` _array_element))
    (bind (_x _y) (`self.GetXandY` _asbp_world_block))
    (if (not (and (== _x (`self.XPosition`)) (== _y (`self.YPosition`))))
      (`KismetArrayLibrary.Array_Add` (`local.SurroundingBlockTypesTemp`) _asbp_world_block)))
  (return (`local.SurroundingBlockTypesTemp`)))

(fn `OnGetIsDecorated`
  (returns (IsDecorated :type Boolean))
  (return (`self.IsDocorated`)))

(fn `OnSetIsDecorated`
  (params (IsDecorated :type Boolean))
  (set `self.IsDocorated` IsDecorated))

(fn `UserConstructionScript`)