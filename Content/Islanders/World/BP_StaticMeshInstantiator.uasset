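; Islanders world Blueprint that batches placed meshes, apparently buildings, into Instanced Static Mesh components created on demand.
; Two events take world transforms: one keys components by mesh using its first material, the other by a supplied material.
; Each event looks up its map, creates a component on a miss, then adds the instance.
; The material path skips recorded transforms for existing components and keeps each component's first mesh.
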(event `OnAddStaticMeshInstanceSortedByMesh`
  (params (TargetTransform :type "Transform Structure") (TargetMesh :type "StaticMesh Object Reference"))
  (bind _currentbuildingmesh (`self.CurrentBuildingMesh`))
  (set `self.CurrentBuildingTransform` TargetTransform)
  (set `self.CurrentBuildingMesh` TargetMesh)
  (if (`.ReturnValue` (`BlueprintMapLibrary.Map_Find` (`self.InstancedMeshesByMesh`) (`self.CurrentBuildingMesh`)))
    ;[1 1 1] Add Static Mesh Instance
    (`InstancedStaticMeshComponent.AddInstanceWorldSpace` (`BlueprintMapLibrary.Map_Find` (`self.InstancedMeshesByMesh`) (`self.CurrentBuildingMesh`)) (`self.CurrentBuildingTransform`))
    (else
      ;[1 1 1] If static mesh don´t exist create a new one
      (bind _returnvalue (`AddComponent|NODE_AddInstancedStaticMeshComponent-1`))
      (`StaticMeshComponent.SetStaticMesh` _returnvalue _currentbuildingmesh)
      (`PrimitiveComponent.SetMaterial` _returnvalue 0 (`StaticMesh.GetMaterial` _currentbuildingmesh 0))
      (`BlueprintMapLibrary.Map_Add` (`self.InstancedMeshesByMesh`) (`self.CurrentBuildingMesh`) _returnvalue)
      (`InstancedStaticMeshComponent.AddInstanceWorldSpace` _returnvalue (`self.CurrentBuildingTransform`)))))

(event `OnAddStaticMeshInstanceSortedByMaterial`
  (params (TargetTransform :type "Transform Structure") (TargetMesh :type "StaticMesh Object Reference") (TargetMaterial :type "MaterialInterface Object Reference"))
  (bind _currentbuildingtransform (`self.CurrentBuildingTransform`))
  (bind _currentbuildingtransform_2 (`self.CurrentBuildingTransform`))
  (set `self.CurrentBuildingTransform` TargetTransform)
  (set `self.CurrentBuildingMesh` TargetMesh)
  (set `self.CurrentMaterial` TargetMaterial)
  (if (`.ReturnValue` (`BlueprintMapLibrary.Map_Find` (`self.InstancedMeshesByMaterial`) (`self.CurrentMaterial`)))
    ;[1 1 1] Add Static Mesh Instance
    (if (not (`KismetArrayLibrary.Array_Contains` (`self.TransformList`) (`self.CurrentBuildingTransform`)))
      (`InstancedStaticMeshComponent.AddInstanceWorldSpace` (`BlueprintMapLibrary.Map_Find` (`self.InstancedMeshesByMaterial`) (`self.CurrentMaterial`)) _currentbuildingtransform)
      (`KismetArrayLibrary.Array_Add` (`self.TransformList`) _currentbuildingtransform))
    (else
      ;[1 1 1] If static mesh don´t exist create a new one
      (bind _returnvalue (`AddComponent|NODE_AddInstancedStaticMeshComponent-0`))
      (`StaticMeshComponent.SetStaticMesh` _returnvalue (`self.CurrentBuildingMesh`))
      (`PrimitiveComponent.SetMaterial` _returnvalue 0 (`self.CurrentMaterial`))
      (`BlueprintMapLibrary.Map_Add` (`self.InstancedMeshesByMaterial`) (`self.CurrentMaterial`) _returnvalue)
      (`InstancedStaticMeshComponent.AddInstanceWorldSpace` _returnvalue _currentbuildingtransform_2)
      (`KismetArrayLibrary.Array_Add` (`self.TransformList`) _currentbuildingtransform_2))))

(fn `UserConstructionScript`)