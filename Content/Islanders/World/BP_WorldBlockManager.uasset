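; BP_WorldBlockManager creates collision volumes for world blocks, with no block meshes or other logic in this graph.
; Its spawn event adds a small box component at the given position, visible in game and tagged with the block type's enum name.
; Each box generates overlaps, has query-and-physics collision on a custom object channel, and blocks that channel plus a second custom trace channel.
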(event `OnSpawnWorldBlockBoxCollider`
  (params (Pos :type "Vector Structure") (WorldBlockType :type "/Game/Islanders/World/E_WorldBlockType Enum" :default "NewEnumerator0"))
  (bind _returnvalue (`AddComponent|NODE_AddBoxComponent-0` :`RelativeTransform` (`KismetMathLibrary.MakeTransform` Pos (struct) (0.2 0.2 0.2))))
  (`BoxComponent.SetBoxExtent` _returnvalue (50.0 50.0 50.0) false)
  (set `PrimitiveComponent.bGenerateOverlapEvents` true _returnvalue)
  (`SceneComponent.SetHiddenInGame` _returnvalue false false)
  (set `ActorComponent.ComponentTags` (`|MakeArray` (`KismetStringLibrary.Conv_StringToName` (`|GetEnumeratorNameAsString` WorldBlockType))) _returnvalue)
  (`PrimitiveComponent.SetCollisionEnabled` _returnvalue "QueryAndPhysics")
  (`PrimitiveComponent.SetCollisionObjectType` _returnvalue "ECC_GameTraceChannel2")
  (`PrimitiveComponent.SetCollisionResponseToChannel` _returnvalue "ECC_GameTraceChannel1" "ECR_Block")
  (`PrimitiveComponent.SetCollisionResponseToChannel` _returnvalue "ECC_GameTraceChannel2" "ECR_Block"))

(fn `UserConstructionScript`)