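; BP_BuildingEffect is a pooled actor that plays the scale-up placement animation for a newly constructed building.
; On start it takes the given mesh, waits a short random delay, then shows and grows it from half to full size along a timeline.
; When finished it hides the mesh, hands it to the Instansiator as a static mesh instance, parks itself off-site and unsubscribes from the BuildingManager's active effect pool.
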(event `OnStartBuildingEffect`
  (params (Building :type "StaticMesh Object Reference") (Instansiator :type "/Game/Islanders/World/BP_StaticMeshInstantiator Object Reference") (BuildingManager :type "/Game/Islanders/Construction/BP_BuildingManager Object Reference"))
  (bind _buildingmesh (`self.BuildingMesh`))
  (`StaticMeshComponent.SetStaticMesh` (`self.BuildingMesh`) Building)
  (set `self.isActive` true)
  (`SceneComponent.SetRelativeScale3D` (`self.BuildingMesh`) (0.5 0.5 0.5))
  (`KismetSystemLibrary.Delay` (`KismetMathLibrary.RandomFloatInRange` 0.0 0.15))
  (`SceneComponent.SetVisibility` (`self.BuildingMesh`) true false)
  (bind (_direction _alpha) (`Timeline|PlaceEffect` :!via `PlayFromStart`)
    (:`Update`
      (`SceneComponent.SetRelativeScale3D` (`self.BuildingMesh`) (`KismetMathLibrary.VLerp` (0.5 0.5 0.5) (1.0 1.0 1.0) _alpha)))
    (:`Finished`
      (`SceneComponent.SetVisibility` (`self.BuildingMesh`) false false)
      (`/Game/Islanders/World/BP_StaticMeshInstantiator.OnAddStaticMeshInstanceSortedByMesh` Instansiator (`SceneComponent.K2_GetComponentToWorld` _buildingmesh) (`StaticMeshComponent.StaticMesh` _buildingmesh))
      (`self.K2_SetActorLocation` (-1000.0 -1000.0 -1000.0))
      (`/Game/Islanders/Construction/BP_BuildingManager.OnUnSubscribeFromACtiveEffectPool` BuildingManager self))))

(fn `UserConstructionScript`)