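; Base Blueprint for world artifacts that, while active, accumulate points toward a required level and return any excess to the caller.
; Instantiation sets mesh and particles by rarity, plays a scale-in timeline and links the world widget ArtifactUI, whose update callbacks toggle the burst particle.
; The widget shows progress, self-resetting point forecasts and hover info, and yaw-rotates with the player camera.
; Depletion is stubbed, and child hover hooks are empty.
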(event `OnEnableArtifacts`
  (params (Enable :type Boolean))
  ;[1 1 1] Disable and enable Artifacts
  ;;[1 1 1] WBP_HUD
  (if Enable
    (set `self.Active` true)
    (`/Game/Islanders/Artifacts/WBP_ArtifactUI.OnSetActive` (`self.ArtifactUI`) true)
    (else
      (set `self.Active` false)
      (`/Game/Islanders/Artifacts/WBP_ArtifactUI.OnSetActive` (`self.ArtifactUI`) false))))

(event `OnResetTextToArtifactLevel`
  ;[1 1 1] Set text back to normal when building detection sphere don´t overlap
  ;;[1 1 1] BP_Player
  (if (`self.Active`)
    (`KismetSystemLibrary.RetriggerableDelay` 0.1)
    (`/Game/Islanders/Artifacts/WBP_ArtifactUI.OnRestForecast` (`self.ArtifactUI`))))

(event `OnIsDepleted`
  ;[1 1 1] Depleted Artifact
  (`KismetSystemLibrary.PrintString` "Hello there artifact" true true (struct :`G` 0.66 :`B` 1.0 :`A` 1.0) 50.0))

(event `OnCompletInstansiation`
  ;[1 1 1] Instansiate
  (`|ExecutionSequence` :!label _label
    (:`then_0`
      (bind _ashighlander_instance (cast `/Game/Islanders/Game/HighlanderInstance` (`GameplayStatics.GetGameInstance`)))
      (set `self.GameInstance` _ashighlander_instance))
    (:`then_1`
      (set `self.TextStartSize` (`SceneComponent.RelativeScale3D` (`self.ArtifactLevelText`))))
    (:`then_2`
      (`TextRenderComponent.K2_SetText` (`self.ArtifactLevelText`) (`KismetTextLibrary.Conv_IntToText` (`self.ArtifactLevel`))))
    (:`then_3`
      (bind _aswbp_artifact_ui (cast `/Game/Islanders/Artifacts/WBP_ArtifactUI` (`WidgetComponent.GetUserWidgetObject` (`self.UI`))))
      (set `self.ArtifactUI` _aswbp_artifact_ui))
    (:`then_4`
      (switch `MyRarity` (`self.Rarity`)
        (:`R_Negative`
          (`StaticMeshComponent.SetStaticMesh` (`self.SM_Artifact`) (`|GetArrayItem` (`.RaritiesApperence_9_B922ED5F49DDBB13780A87AB7C73B23E` (break `/Game/Islanders/Artifacts/S_ArtifactRarityApperence` (`self.RarityApperence`)))) :!label _label_2)
          (`ParticleSystemComponent.SetTemplate` (`self.BurstParticle`) "/Game/Islanders/Artifacts/P_Artifact_Burst_C.P_Artifact_Burst_C")
          (`ParticleSystemComponent.SetTemplate` (`self.ParticleIdle`) "/Game/Islanders/Artifacts/P_Artifact_C.P_Artifact_C"))
        (:`R_Common`
          (goto _label_2))
        (:`R_UnCommon`
          (`StaticMeshComponent.SetStaticMesh` (`self.SM_Artifact`) (`|GetArrayItem` (`.RaritiesApperence_9_B922ED5F49DDBB13780A87AB7C73B23E` (break `/Game/Islanders/Artifacts/S_ArtifactRarityApperence` (`self.RarityApperence`))) 1))
          (`ParticleSystemComponent.SetTemplate` (`self.BurstParticle`) "/Game/Islanders/Artifacts/P_Artifact_Burst_UC.P_Artifact_Burst_UC")
          (`ParticleSystemComponent.SetTemplate` (`self.ParticleIdle`) "/Game/Islanders/Artifacts/P_Artifact_UC.P_Artifact_UC"))
        (:`R_Rare`
          (`StaticMeshComponent.SetStaticMesh` (`self.SM_Artifact`) (`|GetArrayItem` (`.RaritiesApperence_9_B922ED5F49DDBB13780A87AB7C73B23E` (break `/Game/Islanders/Artifacts/S_ArtifactRarityApperence` (`self.RarityApperence`))) 2))
          (`ParticleSystemComponent.SetTemplate` (`self.BurstParticle`) "/Game/Islanders/Artifacts/P_Artifact_Burst_R.P_Artifact_Burst_R")
          (`ParticleSystemComponent.SetTemplate` (`self.ParticleIdle`) "/Game/Islanders/Artifacts/P_Artifact_R.P_Artifact_R"))
        (:`R_Legendary`
          (`StaticMeshComponent.SetStaticMesh` (`self.SM_Artifact`) (`|GetArrayItem` (`.RaritiesApperence_9_B922ED5F49DDBB13780A87AB7C73B23E` (break `/Game/Islanders/Artifacts/S_ArtifactRarityApperence` (`self.RarityApperence`))) 3))
          (`ParticleSystemComponent.SetTemplate` (`self.BurstParticle`) "/Game/Islanders/Artifacts/P_Artifact_Burst_L.P_Artifact_Burst_L")
          (`ParticleSystemComponent.SetTemplate` (`self.ParticleIdle`) "/Game/Islanders/Artifacts/P_Artifact_L.P_Artifact_L"))))
    (:`then_5`
      (add `/Game/Islanders/Artifacts/WBP_ArtifactUI.StartUpdate` (`self.ArtifactUI`) (delegate `OnCallStartUIUpdate`))
      (add `/Game/Islanders/Artifacts/WBP_ArtifactUI.EndUpdate` (`self.ArtifactUI`) (delegate `OnCallEndUIUpdate`)))
    (:`then_6`
      (bind (_direction _alpha) (`Timeline|SpawnEffect` :!via `PlayFromStart`)
        (:`Update`
          (`SceneComponent.SetRelativeScale3D` (`self.SM_Artifact`) (`KismetMathLibrary.VLerp` (0.2 0.2 0.2) (`self.StaticMeshStartScale`) _alpha)))
        (:`Finished`
          (`/Game/Islanders/Artifacts/WBP_ArtifactUI.OnPlaySpawnAnim` (`self.ArtifactUI`)))))))

(event `OnInstnasiate`
  (params (HUD :type "/Game/Islanders/Player/WBP_HUD Object Reference") (WorldGenerator :type "/Game/Islanders/World/BP_myWorldGenerator Object Reference") (ArtifactType :type "MyArtifactTypes Enum" :default "AT_WorldGeneration") (ArtifactLevel :type Integer) (`Pop Up` :type "/Game/Islanders/Player/WBP_PopUp Object Reference") (X :type Integer) (Y :type Integer) (Rarities :type "MyRarity Enum" :default "R_Negative"))
  ;[1 1 1] Instansiate
  (set `self.HUD` HUD)
  (set `self.WorldGenerator` WorldGenerator)
  (set `self.ArtifactType` ArtifactType)
  (set `self.ArtifactLevel` ArtifactLevel)
  (set `self.PopUp` `Pop Up`)
  (set `self.StaticMeshStartScale` (`SceneComponent.RelativeScale3D` (`self.ArtifactLevelText`)))
  (set `self.X` X)
  (set `self.Y` Y)
  (set `self.Rarity` Rarities)
  (set `self.StartingRotation` (`SceneComponent.RelativeRotation` (`self.UI`)))
  (goto _label))

(event `OnHoverOverChildren`
  ;[1 1 1] Pop up for artifacts
)

(event `OnEndHoverOverChildren`
  ;[1 1 1] Pop up for artifacts
)

(event `self.Box.OnBeginCursorOver`
  (params (TouchedComponent :type "PrimitiveComponent Object Reference"))
  ;[1 1 1] Pop up for artifacts
  (`self.OnHoverOverChildren`)
  (`/Game/Islanders/Artifacts/WBP_ArtifactUI.OnShowExtraInfo` (`self.ArtifactUI`))
  (if (not (`self.Active`))
    (`/Game/Islanders/Artifacts/WBP_ArtifactUI.OnSetActive` (`self.ArtifactUI`) true)))

(event `OnRotateText`
  (params (ZRotCameraOffset :type "Float (double-precision)"))
  (bind (_startingrotation_roll _startingrotation_pitch _startingrotation_yaw) (`KismetMathLibrary.BreakRotator` (`self.StartingRotation`)))
  (bind _returnvalue (`KismetMathLibrary.MakeRotator` _startingrotation_roll _startingrotation_pitch (+ _startingrotation_yaw ZRotCameraOffset)))
  ;[1 1 1] Rotate the text to face the player
  ;;[1 1 1] BP_Player
  (`SceneComponent.K2_SetRelativeRotation` (`self.ArtifactLevelText`) _returnvalue false false)
  (`SceneComponent.K2_SetRelativeRotation` (`self.UI`) _returnvalue false false))

(event `self.Box.OnEndCursorOver`
  (params (TouchedComponent :type "PrimitiveComponent Object Reference"))
  ;[1 1 1] Pop up for artifacts
  (`self.OnEndHoverOverChildren`)
  (`/Game/Islanders/Artifacts/WBP_ArtifactUI.OnHideExtraInfo` (`self.ArtifactUI`))
  (if (`self.Active`)
    (`/Game/Islanders/Artifacts/WBP_ArtifactUI.OnSetActive` (`self.ArtifactUI`) true)
    (else
      (`/Game/Islanders/Artifacts/WBP_ArtifactUI.OnSetActive` (`self.ArtifactUI`) false))))

(event `OnCallStartUIUpdate`
  ;[1 1 1] Instansiate
  (`self.OnStartUIUpdate`))

(event `OnCallEndUIUpdate`
  ;[1 1 1] Instansiate
  (`self.OnEndUIUpdate`))

(event `OnStartUIUpdate`
  (`ActorComponent.Activate` (`self.BurstParticle`) true))

(event `OnEndUIUpdate`
  (`ActorComponent.Deactivate` (`self.BurstParticle`)))

(event `OnHideUI`
  (params (Hide :type Boolean))
  ;[1 1 1] Hide UI for Artifact UI
  (if Hide
    (`SceneComponent.SetVisibility` (`self.UI`) false false)
    (else
      (`SceneComponent.SetVisibility` (`self.UI`) true false))))

(fn `Instansiation`
  (params (HUD :type "/Game/Islanders/Player/WBP_HUD Object Reference") (WorldGenerator :type "/Game/Islanders/World/BP_myWorldGenerator Object Reference") (ArtifactType :type "MyArtifactTypes Enum" :default "AT_WorldGeneration") (ArtifactLevel :type Integer) (PopUp :type "/Game/Islanders/Player/WBP_PopUp Object Reference") (X :type Integer) (Y :type Integer) (Rarity :type "MyRarity Enum" :default "R_Negative"))
  (set `self.HUD` HUD)
  (set `self.WorldGenerator` WorldGenerator)
  (set `self.ArtifactType` ArtifactType)
  (set `self.ArtifactLevel` ArtifactLevel)
  (set `self.PopUp` PopUp)
  (set `self.StaticMeshStartScale` (`SceneComponent.RelativeScale3D` (`self.ArtifactLevelText`)))
  (set `self.StartingRotation` (`SceneComponent.RelativeRotation` (`self.UI`)))
  (set `self.X` X)
  (set `self.Y` Y)
  (set `self.Rarity` Rarity)
  (`self.OnCompletInstansiation`))

(fn `On ShowArtifact LevelForcast`
  (params (points :type Integer))
  (returns (PointsLeftOver :type Integer))
  (locals (TempArtifactLevelFocast :type Integer) (PointsTemp :type Integer))
  (set `local.PointsTemp` points)
  (if (`self.Active`)
    (`|ExecutionSequence`
      (:`then_0`
        ;[1 1 1] Set Text
        (`/Game/Islanders/Artifacts/WBP_ArtifactUI.OnUpdateForecast` (`self.ArtifactUI`) (`local.PointsTemp`)))
      (:`then_2`
        (`self.OnResetTextToArtifactLevel`))
      (:`then_3`
        (if (> (`self.ArtifactLevel`) (+ (`local.PointsTemp`) (`self.CurrentArtifactLevel`)))
          (return 0)
          (else
            (return (- (+ (`local.PointsTemp`) (`self.CurrentArtifactLevel`)) (`self.ArtifactLevel`)))))))
    (else
      (return (`local.PointsTemp`)))))

(fn `OnDepleted`)

(fn `OnUpdateArtifactLevel`
  (params (Points :type Integer))
  (returns (LeftOverPoints :type Integer))
  (locals (LeftOverPointsTemp :type Integer) (PointsTemp :type Integer))
  (bind _output_get (set `local.PointsTemp` Points))
  (if (`self.Active`)
    (set `self.CurrentArtifactLevel` (+ (`self.CurrentArtifactLevel`) _output_get))
    (`/Game/Islanders/Artifacts/WBP_ArtifactUI.OnUpdateProgressBar` (`self.ArtifactUI`) (`self.CurrentArtifactLevel`))
    (if (> (`self.ArtifactLevel`) (`self.CurrentArtifactLevel`))
      (return 0)
      (else
        (return (- (`self.CurrentArtifactLevel`) (`self.ArtifactLevel`)))))
    (else
      (return (`local.PointsTemp`)))))

(fn `UserConstructionScript`)