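; Artifact actor that, when depleted, expands the world at the closest position with terrain of its generation type.
; On setup, it initializes its UI widget, binds depletion and land-unlock events, and derives block-count range, bonus blocks and natural-resource modifier from rarity and type.
; Depletion fires once, requesting the expansion, removing the artifact from the ascension manager, then shrinking and hiding the mesh.
; Hover-end closes the pop-up, but its activation call is disconnected.
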(event `OnHoverOverChildren_1`
  ;[1 1 1] Pop Up
  (`|ExecutionSequence`
    (:`then_0`
      (`KismetSystemLibrary.Delay` 0.2)
      (`/Engine/EditorBlueprintResources/StandardMacros.Gate` true :!label _label))
    (:`then_1`
      (goto _label :!via `Open`))))

(event `OnSetStartingProperties`
  (params (GenerationType :type "MyArtifactGenerationType Enum" :default "AGT_RockyGrassLands"))
  ;[1 1 1] Set Properties
  (set `self.MyGenerationType` GenerationType)
  (`|ExecutionSequence`
    (:`then_0`
      (bind _aswbp_artifact_ui (cast `/Game/Islanders/Artifacts/WBP_ArtifactUI` (`WidgetComponent.GetUserWidgetObject` (`self.UI`))))
      (`/Game/Islanders/Artifacts/WBP_ArtifactUI.Instansiate` _aswbp_artifact_ui "AT_WorldGeneration" (`self.Rarity`) (`self.ArtifactLevel`) "Tree"))
    (:`then_1`
      (add `/Game/Islanders/Artifacts/WBP_ArtifactUI.ArtifactIsDepleted` (`self.ArtifactUI`) (delegate `CallOnIsDepeted`))
      (add `/Game/Islanders/Artifacts/WBP_ArtifactUI.willCompleteArtifact` (`self.ArtifactUI`) (delegate `CallUnlockNewLand`)))
    (:`then_2`
      (switch `MyRarity` (`self.Rarity`)
        (:`R_Common`
          (set `self.MinBlockCount` 10)
          (set `self.MaxBlockCount` 15)
          (set `self.NaturalRecurcesModifiers` 1.1))
        (:`R_UnCommon`
          (set `self.MinBlockCount` 20)
          (set `self.MaxBlockCount` 25)
          (set `self.NaturalRecurcesModifiers` 1.2))
        (:`R_Rare`
          (set `self.MinBlockCount` 30)
          (set `self.MaxBlockCount` 40)
          (set `self.NaturalRecurcesModifiers` 1.35))
        (:`R_Legendary`
          (set `self.MinBlockCount` 50)
          (set `self.MaxBlockCount` 70)
          (set `self.NaturalRecurcesModifiers` 1.5))))
    (:`then_3`
      (switch `MyRarity` (`self.Rarity`)
        (:`R_Common`
          (switch `MyArtifactGenerationType` (`self.MyGenerationType`) :!label _label_2
            (:`AGT_RockyGrassLands`
              (set `self.GenTypeAdditionBlockCount` 0))
            (:`AGT_GrassLands`
              (set `self.GenTypeAdditionBlockCount` 10))
            (:`AGT_RockLands`
              (set `self.GenTypeAdditionBlockCount` 0))
            (:`AGT_BigLake`
              (set `self.GenTypeAdditionBlockCount` 10))
            (:`AGT_SmallArtifactArea`
              (set `self.GenTypeAdditionBlockCount` 0))
            (:`AGT_Tarn`
              (set `self.GenTypeAdditionBlockCount` 0))))
        (:`R_UnCommon`
          (goto _label_2))
        (:`R_Rare`
          (switch `MyArtifactGenerationType` (`self.MyGenerationType`) :!label _label_3
            (:`AGT_RockyGrassLands`
              (set `self.GenTypeAdditionBlockCount` 10))
            (:`AGT_GrassLands`
              (set `self.GenTypeAdditionBlockCount` 25))
            (:`AGT_RockLands`
              (set `self.GenTypeAdditionBlockCount` 0))
            (:`AGT_BigLake`
              (set `self.GenTypeAdditionBlockCount` 25))
            (:`AGT_SmallArtifactArea`
              (set `self.GenTypeAdditionBlockCount` 0))
            (:`AGT_Tarn`
              (set `self.GenTypeAdditionBlockCount` 10))))
        (:`R_Legendary`
          (goto _label_3))))))

(event `OnEndHoverOVerChildren_1`
  ;[1 1 1] Pop Up
  (`/Game/Islanders/Player/WBP_PopUp.OnDeActivatePopUp` (`self.PopUp`))
  (goto _label :!via `Close`))

(event `CallOnIsDepeted`
  ;[1 1 1] Set Properties
  (`self.OnArtifactIsDepeted`))

(event `CallUnlockNewLand`
  ;[1 1 1] Set Properties
  (`/Game/Islanders/Player/WBP_HUD.OnUnlockNewLand` (`self.HUD`) (`self.WorldGenerator`)))

(event `OnArtifactIsDepeted`
  ;[1 1 1] Deplet artifact
  (clear `/Game/Islanders/Artifacts/WBP_ArtifactUI.ArtifactIsDepleted` (`self.ArtifactUI`))
  (`/Engine/EditorBlueprintResources/StandardMacros.DoOnce` false
    (:`Completed`
      (`|ExecutionSequence`
        (:`then_0`
          (`self.OnIsDepleted`)
          (set `self.TempBlockCount` (+ (`KismetMathLibrary.RandomIntegerInRange` (`self.MinBlockCount`) (`self.MaxBlockCount`)) (`self.GenTypeAdditionBlockCount`)))
          (`MyWorldGenerator.expandWorldAtClosestPosition` (`self.WorldGenerator`) (`self.X`) (`self.Y`) false (`self.MyGenerationType`) (`self.TempBlockCount`) (`self.NaturalRecurcesModifiers`)))
        (:`then_1`
          (`MyWorldGenerator.OnRemoveArtifactInAscensionManager` (`self.WorldGenerator`) (`self.ArtifactType`)))
        (:`then_2`
          (bind (_direction _alpha) (`Timeline|Timeline_0` :!via `ReverseFromEnd`)
            (:`Update`
              (`SceneComponent.SetRelativeScale3D` (`self.SM_Artifact`) (`KismetMathLibrary.VLerp` (0.2 0.2 0.2) (`self.StaticMeshStartScale`) _alpha)))
            (:`Finished`
              (`self.SetActorHiddenInGame` true)
              (`PrimitiveComponent.SetCollisionEnabled` (`self.Box`) "NoCollision"))))))))

(event `self.OnIsDepleted`
  ;[1 1 1] Deplet artifact
)

(fn `UserConstructionScript`
  (`parent.UserConstructionScript`))