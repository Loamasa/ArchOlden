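; Modifier artifact actor, a child artifact that grants a named modifier of a given rarity to the player when depleted.
; Its starting properties initialise the artifact UI widget and bind to that UI's depletion event.
; Depletion adds the modifier to the game instance and HUD, hides the actor, disables collision and has the world generator deregister it.
; Hover drives a delayed gate, but the pop-up activation is unwired; ending hover deactivates the pop-up.
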(event `self.OnHoverOverChildren`
  ;[1 1 1] Pop Up
  (`|ExecutionSequence`
    (:`then_0`
      (`KismetSystemLibrary.Delay` 0.2)
      (`/Engine/EditorBlueprintResources/StandardMacros.Gate` true :!label _label))
    (:`then_1`
      (goto _label :!via `Open`))))

(event `OnSetStartingProperties`
  (params (ModifierName :type String) (Rarity :type "MyRarity Enum" :default "R_Negative"))
  ;[1 1 1] Set Starting Properties
  (set `self.ModifierName` ModifierName)
  (set `self.Rarity_0` Rarity)
  (bind _aswbp_artifact_ui (cast `/Game/Islanders/Artifacts/WBP_ArtifactUI` (`WidgetComponent.GetUserWidgetObject` (`self.UI`))))
  (`/Game/Islanders/Artifacts/WBP_ArtifactUI.Instansiate` _aswbp_artifact_ui "AT_Modifier" (`self.Rarity_0`) (`self.ArtifactLevel`) "Tree")
  (add `/Game/Islanders/Artifacts/WBP_ArtifactUI.ArtifactIsDepleted` (`self.ArtifactUI`) (delegate `CallOnIsDepeted`)))

(event `self.OnEndHoverOVerChildren`
  ;[1 1 1] Pop Up
  (`/Game/Islanders/Player/WBP_PopUp.OnDeActivatePopUp` (`self.PopUp`))
  (goto _label :!via `Close`))

(event `CallOnIsDepeted`
  ;[1 1 1] Set Starting Properties
  (`self.OnArtifactIsDepeted`))

(event `OnArtifactIsDepeted`
  ;[1 1 1] Deplet artifact
  (clear `/Game/Islanders/Artifacts/WBP_ArtifactUI.ArtifactIsDepleted` (`self.ArtifactUI`))
  (`|ExecutionSequence`
    (:`then_0`
      (`/Game/Islanders/Game/HighlanderInstance.Add Modifier` (`self.GameInstance`) (`self.ModifierName`) (`self.Rarity_0`))
      (`/Game/Islanders/Player/WBP_HUD.OnAddModifierIcon` (`self.HUD`) (`self.ModifierName`) (`self.Rarity_0`)))
    (:`then_1`
      (`self.SetActorHiddenInGame` true)
      (`PrimitiveComponent.SetCollisionEnabled` (`self.Box`) "NoCollision"))
    (:`then_2`
      (`MyWorldGenerator.OnRemoveArtifactInAscensionManager` (`self.WorldGenerator`) (`self.ArtifactType`)))))

(event `self.OnIsDepleted`
  ;[1 1 1] Deplet artifact
)

(fn `Instansiation`
  (params (HUD :type "/Game/Islanders/Player/WBP_HUD Object Reference") (WorldGenerator :type "/Game/Islanders/World/BP_myWorldGenerator Object Reference") (ArtifactType :type "MyArtifactTypes Enum" :default "AT_WorldGeneration") (ArtifactLevel :type Integer) (PopUp :type "/Game/Islanders/Player/WBP_PopUp Object Reference") (X :type Integer) (Y :type Integer) (Rarity :type "MyRarity Enum" :default "R_Negative"))
  (`parent.Instansiation` HUD WorldGenerator ArtifactType ArtifactLevel PopUp X Y "R_Negative"))

(fn `UserConstructionScript`
  (`parent.UserConstructionScript`))