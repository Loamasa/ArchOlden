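; Building artifact actor that, once depleted, adds its building type to the player's hand through the HUD.
; On setup it stores the type, initializes its artifact UI widget and binds that widget's depleted and will-complete events.
; Depletion also shrinks the mesh with a reversed timeline, then hides the actor and disables box collision; imminent completion notifies the HUD.
; Hover end closes the pop-up, but the delayed, gated hover-start path activates nothing.
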(event `OnHoverOver`)

(event `OnArtifactIsDepletedDirect`
  ;[1 1 1] Deplet artifact
)

(event `self.OnHoverOverChildren`
  ;[1 1 1] Pop Up
  (`|ExecutionSequence`
    (:`then_0`
      (`KismetSystemLibrary.Delay` 0.2)
      (`/Engine/EditorBlueprintResources/StandardMacros.Gate` true :!label _label))
    (:`then_1`
      (goto _label :!via `Open`))))

(event `OnSetStartingProperties`
  (params (BuildingType :type "MyBuildingType Enum" :default "Tree"))
  ;[1 1 1] Set Properties
  (bind _output_get (set `self.BuildingType` BuildingType))
  (bind _mybuildingdata (`/Game/Islanders/Game/HighlanderInstance.CSV GetBuildingData` (`self.GameInstance`) _output_get))
  (set `self.MyRarity` (`.Rarity` (break `MyBuildingData` _mybuildingdata)))
  (bind _aswbp_artifact_ui (cast `/Game/Islanders/Artifacts/WBP_ArtifactUI` (`WidgetComponent.GetUserWidgetObject` (`self.UI`))))
  (`/Game/Islanders/Artifacts/WBP_ArtifactUI.Instansiate` _aswbp_artifact_ui "AT_Building" "R_Common" (`self.ArtifactLevel`) (`self.BuildingType`))
  (add `/Game/Islanders/Artifacts/WBP_ArtifactUI.ArtifactIsDepleted` (`self.ArtifactUI`) (delegate `CallOnIsDepeted`))
  (add `/Game/Islanders/Artifacts/WBP_ArtifactUI.willCompleteArtifact` (`self.ArtifactUI`) (delegate `CallWillBeCompleted`)))

(event `OnArtifactIsDepeted`
  ;[1 1 1] Deplet artifact
  (`|ExecutionSequence`
    (:`then_0`
      (`/Game/Islanders/Player/WBP_HUD.OnAddBuildingToHand` (`self.HUD`) (`self.BuildingType`)))
    (:`then_2`
      (bind (_direction _alpha) (`Timeline|Timeline_0` :!via `ReverseFromEnd`)
        (:`Update`
          (`SceneComponent.SetRelativeScale3D` (`self.SM_Artifact`) (`KismetMathLibrary.VLerp` (0.2 0.2 0.2) (`self.StaticMeshStartScale`) _alpha)))
        (:`Finished`
          (`self.SetActorHiddenInGame` true)
          (`PrimitiveComponent.SetCollisionEnabled` (`self.Box`) "NoCollision"))))))

(event `self.OnEndHoverOVerChildren`
  ;[1 1 1] Pop Up
  (`/Game/Islanders/Player/WBP_PopUp.OnDeActivatePopUp` (`self.PopUp`))
  (goto _label :!via `Close`))

(event `CallOnIsDepeted`
  ;[1 1 1] Set Properties
  (`self.OnArtifactIsDepeted`))

(event `CallWillBeCompleted`
  ;[1 1 1] Set Properties
  (`/Game/Islanders/Player/WBP_HUD.OnArtifactWillComplet` (`self.HUD`)))

(fn `UserConstructionScript`
  (`parent.UserConstructionScript`))