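; BP_Artifact_Wincondition is the artifact variant that ends the game in a win when depleted.
; Instansiation extends the parent's, sets the artifact UI widget to the Win type and binds its depletion event.
; On depletion it unbinds that event and calls OnWinGame on the HUD.
; Hover opens a delayed gate with no connected output, leaving the win popup unreachable, while ending hover closes the popup.
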(event `OnArtifactIsDepeted`
  (clear `/Game/Islanders/Artifacts/WBP_ArtifactUI.ArtifactIsDepleted` (`self.ArtifactUI`))
  (`/Game/Islanders/Player/WBP_HUD.OnWinGame` (`self.HUD`)))

(event `self.OnIsDepleted`)

(event `self.OnHoverOverChildren`
  (`|ExecutionSequence`
    (:`then_0`
      (`KismetSystemLibrary.Delay` 0.2)
      (`/Engine/EditorBlueprintResources/StandardMacros.Gate` true :!label _label))
    (:`then_1`
      (goto _label :!via `Open`))))

(event `OnInstansiate`
  (add `/Game/Islanders/Artifacts/WBP_ArtifactUI.ArtifactIsDepleted` (`self.ArtifactUI`) (delegate `CallOnIsDepeted`)))

(event `self.OnEndHoverOVerChildren`
  (`/Game/Islanders/Player/WBP_PopUp.OnDeActivatePopUp` (`self.PopUp`))
  (goto _label :!via `Close`))

(event `CallOnIsDepeted`
  (`self.OnArtifactIsDepeted`))

(fn `Instansiation`
  (params (HUD :type "/Game/Islanders/Player/WBP_HUD Object Reference") (WorldGenerator :type "/Game/Islanders/World/BP_myWorldGenerator Object Reference") (ArtifactType :type "MyArtifactTypes Enum" :default "AT_WorldGeneration") (ArtifactLevel :type Integer) (PopUp :type "/Game/Islanders/Player/WBP_PopUp Object Reference") (X :type Integer) (Y :type Integer) (Rarity :type "MyRarity Enum" :default "R_Negative"))
  (`parent.Instansiation` HUD WorldGenerator ArtifactType ArtifactLevel PopUp X Y "R_Negative")
  (bind _aswbp_artifact_ui (cast `/Game/Islanders/Artifacts/WBP_ArtifactUI` (`WidgetComponent.GetUserWidgetObject` (`self.UI`))))
  (`/Game/Islanders/Artifacts/WBP_ArtifactUI.Instansiate` _aswbp_artifact_ui "AT_Win" "R_Negative" (`local.ArtifactLevel`) "Tree")
  (`self.OnInstansiate`))

(fn `UserConstructionScript`
  (`parent.UserConstructionScript`))