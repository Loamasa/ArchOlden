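; BP_CSVData is a data container for imported CSV game data: buildings, rarities, placement profiles, modifiers, per-region artifact generation, difficulty compatibility matrices and building appearances.
; OnSetCSVData copies every imported dataset into member variables, with no parsing or validation.
; Three getters expose the stored data: GetCSV for the core and artifact tables, OnGetDifficultiesMatrix for the Easy-to-Extreme matrices, and GetBuildingApperences for appearances.
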(event `OnSetCSVData`
  (params (ImportedCSVBuildingData :type "Map of MyBuildingType Enum to MyBuildingData Structure") (ImportedCSVRaritiesData :type "Map of MyRarity Enum to /Game/Islanders/Core/Rarity/S_RarityData Structure") (ImportedCSVPlacmentProfile :type "Map of MyPlacmentProfile Enum to /Game/Islanders/Construction/S_PlacmentProfile Structure") (ImportedCSVModifiersData :type "Map of String to MyModifierData Structure") (ImportedCSVModifiersNames :type "Array of String") (ImportedCSVArtifactGenerationRockyPlains :type "Array of MyWorldGenerationData Structure") (ImportedCSVArtifactGenerationDataPlains :type "Array of MyWorldGenerationData Structure") (ImportedCSVArtifactGenerationRockLands :type "Array of MyWorldGenerationData Structure") (ImportedCSVArtifactGenerationBigLake :type "Array of MyWorldGenerationData Structure") (ImportedCSVArtifactGenerationSmallArtifactArea :type "Array of MyWorldGenerationData Structure") (ImportedCSVArtifactGenerationTarn :type "Array of MyWorldGenerationData Structure") (ImportedCSVEasyCompatabilityMatrix :type "Array of MyCompatibilities Structure") (ImportedCSVNormalCompatabilityMatrix :type "Array of MyCompatibilities Structure") (ImportedCSVHardCompatabilityMatrix :type "Array of MyCompatibilities Structure") (ImportedCSVExtremeCompatabilityMatrix :type "Array of MyCompatibilities Structure") (ImportedBuildingApperences :type "Map of MyBuildingType Enum to /Game/Islanders/Construction/S_BuildingApperence Structure"))
  (set `self.CSVBuildingData` ImportedCSVBuildingData)
  (set `self.CSVRaritiesData` ImportedCSVRaritiesData)
  (set `self.CSVPlacmentProfile` ImportedCSVPlacmentProfile)
  (set `self.CSVModifiers` ImportedCSVModifiersData)
  (set `self.CSVModifiersUniqueNames` ImportedCSVModifiersNames)
  (set `self.CSVArtifactGenerationRockyPlains` ImportedCSVArtifactGenerationRockyPlains)
  (set `self.CSVArtifactGenerationDataPlains` ImportedCSVArtifactGenerationDataPlains)
  (set `self.CSVArtifactGenerationRockLands` ImportedCSVArtifactGenerationRockLands)
  (set `self.CSVArtifactGenerationBigLake` ImportedCSVArtifactGenerationBigLake)
  (set `self.CSVArtifactGenerationSmallArtifactArea` ImportedCSVArtifactGenerationSmallArtifactArea)
  (set `self.CSVArtifactGenerationTarn` ImportedCSVArtifactGenerationTarn)
  (set `self.CSVEasyCompatabilityMatrix` ImportedCSVEasyCompatabilityMatrix)
  (set `self.CSVNormalCompatabilityMatrix` ImportedCSVNormalCompatabilityMatrix)
  (set `self.CSVHardCompatabilityMatrix` ImportedCSVHardCompatabilityMatrix)
  (set `self.CSVExtremeCompatabilityMatrix` ImportedCSVExtremeCompatabilityMatrix)
  (set `self.BuildingApperences` ImportedBuildingApperences))

(fn `GetBuildingApperences`
  (returns (ImportedBuildingApperences :type "Map of MyBuildingType Enum to /Game/Islanders/Construction/S_BuildingApperence Structure"))
  (return (`self.BuildingApperences`)))

(fn `GetCSV`
  (returns (BuildingData :type "Map of MyBuildingType Enum to MyBuildingData Structure") (RaritiesData :type "Map of MyRarity Enum to /Game/Islanders/Core/Rarity/S_RarityData Structure") (PlacmentProfile :type "Map of MyPlacmentProfile Enum to /Game/Islanders/Construction/S_PlacmentProfile Structure") (Modifiers :type "Map of String to MyModifierData Structure") (ModifiersName :type "Array of String") (CSVArtifactGenerationRockyPlains :type "Array of MyWorldGenerationData Structure") (CSVArtifactGenerationDataPlains :type "Array of MyWorldGenerationData Structure") (CSVArtifactGenerationRockLands :type "Array of MyWorldGenerationData Structure") (CSVArtifactGenerationBigLake :type "Array of MyWorldGenerationData Structure") (CSVArtifactGenerationSmallArtifactArea :type "Array of MyWorldGenerationData Structure") (CSVArtifactGenerationTarn :type "Array of MyWorldGenerationData Structure"))
  (return (`self.CSVBuildingData`) (`self.CSVRaritiesData`) (`self.CSVPlacmentProfile`) (`self.CSVModifiers`) (`self.CSVModifiersUniqueNames`) (`self.CSVArtifactGenerationRockyPlains`) (`self.CSVArtifactGenerationDataPlains`) (`self.CSVArtifactGenerationRockLands`) (`self.CSVArtifactGenerationBigLake`) (`self.CSVArtifactGenerationSmallArtifactArea`) (`self.CSVArtifactGenerationTarn`)))

(fn `OnGetDifficultiesMatrix`
  (returns (EasyCompatabilityMatrix :type "Array of MyCompatibilities Structure") (NormalCompatabilityMatrix :type "Array of MyCompatibilities Structure") (HardCompatabilityMatrix :type "Array of MyCompatibilities Structure") (ExtremeCompatabilityMatrix :type "Array of MyCompatibilities Structure"))
  (return (`self.CSVEasyCompatabilityMatrix`) (`self.CSVNormalCompatabilityMatrix`) (`self.CSVHardCompatabilityMatrix`) (`self.CSVExtremeCompatabilityMatrix`)))

(fn `UserConstructionScript`)