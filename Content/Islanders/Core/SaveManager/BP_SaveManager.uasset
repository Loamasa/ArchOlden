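; BP_SaveManager centralizes saving and loading for ascension runs, player stats and settings, using three SaveGame slots.
; AscensionSlot holds area data, modifiers, round, previous ascensions and a new-ascension-ready flag, with events and functions to save, query or delete it.
; Most operations load the existing slot or fall back to a fresh SaveGame object, while settings saves always overwrite.
; TrySavePlayerAscensionRecord re-saves an existing record without assigning the higher level.
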(event `OnDeletSavedAscension`
  ;[1 1 1] Delet SavedAscension
  (bind _returnvalue (`GameplayStatics.DoesSaveGameExist` "AscensionSlot"))
  (if _returnvalue
    (bind _returnvalue_2 (`GameplayStatics.DeleteGameInSlot` "AscensionSlot"))))

(event `OnSaveSettings`
  (params (Settings :type "/Game/Islanders/StartMenu/S_Settings Structure"))
  (bind _returnvalue (`GameplayStatics.CreateSaveGameObject` "/Game/Islanders/Core/SaveManager/SG_Settings.SG_Settings_C"))
  (set `/Game/Islanders/Core/SaveManager/SG_Settings.SavedSettingData` Settings _returnvalue)
  (`GameplayStatics.SaveGameToSlot` _returnvalue "SettingSlot"))

(event `OnSaveNewAscensionReady`
  ;[1 1 1] New Ascension is Ready
  (bind _returnvalue (`GameplayStatics.DoesSaveGameExist` "AscensionSlot"))
  (if _returnvalue
    (bind _returnvalue_2 (`GameplayStatics.LoadGameFromSlot` "AscensionSlot"))
    (bind _assg_saved_ascension (cast `/Game/Islanders/Core/SaveManager/SG_SavedAscension` _returnvalue_2))
    (set `/Game/Islanders/Core/SaveManager/SG_SavedAscension.NewAscensionReady` true _assg_saved_ascension)
    (`GameplayStatics.SaveGameToSlot` _assg_saved_ascension "AscensionSlot")
    (else
      (bind _returnvalue_3 (`GameplayStatics.CreateSaveGameObject` "/Game/Islanders/Core/SaveManager/SG_SavedAscension.SG_SavedAscension_C"))
      (set `/Game/Islanders/Core/SaveManager/SG_SavedAscension.NewAscensionReady` true _returnvalue_3)
      (`GameplayStatics.SaveGameToSlot` _returnvalue_3 "AscensionSlot"))))

(event `OnSaveAscension`
  (params (StartingArea :type "Array of MyWorldBlockData Structure") (AscensionData :type "MyAscensionData Structure"))
  ;[1 1 1] Save Ascension
  (set `self.CurrentSavingArea` StartingArea)
  (set `self.CurrentAscensionData` AscensionData)
  (bind _returnvalue (`GameplayStatics.DoesSaveGameExist` "AscensionSlot"))
  (if _returnvalue
    (bind _returnvalue_2 (`GameplayStatics.LoadGameFromSlot` "AscensionSlot"))
    (bind _assg_saved_ascension (cast `/Game/Islanders/Core/SaveManager/SG_SavedAscension` _returnvalue_2))
    (bind _structout (setmembers `MySavedAscensionData` :`StructRef` (`/Game/Islanders/Core/SaveManager/SG_SavedAscension.SavedAscension` _assg_saved_ascension) :`savedAreaData` (`self.CurrentSavingArea`) :`savedAscensionData` (`self.CurrentAscensionData`)))
    (set `/Game/Islanders/Core/SaveManager/SG_SavedAscension.SavedAscension` _structout _assg_saved_ascension)
    (set `/Game/Islanders/Core/SaveManager/SG_SavedAscension.NewAscensionReady` false _assg_saved_ascension)
    (bind _returnvalue_3 (`GameplayStatics.SaveGameToSlot` _returnvalue_2 "AscensionSlot"))
    (else
      (bind _returnvalue_4 (`GameplayStatics.CreateSaveGameObject` "/Game/Islanders/Core/SaveManager/SG_SavedAscension.SG_SavedAscension_C"))
      (bind _structout_2 (setmembers `MySavedAscensionData` :`StructRef` (`/Game/Islanders/Core/SaveManager/SG_SavedAscension.SavedAscension` _returnvalue_4) :`savedAreaData` (`self.CurrentSavingArea`) :`savedAscensionData` (`self.CurrentAscensionData`)))
      (set `/Game/Islanders/Core/SaveManager/SG_SavedAscension.SavedAscension` _structout_2 _returnvalue_4)
      (set `/Game/Islanders/Core/SaveManager/SG_SavedAscension.NewAscensionReady` false _returnvalue_4)
      (bind _returnvalue_5 (`GameplayStatics.SaveGameToSlot` _returnvalue_4 "AscensionSlot")))))

(event `OnLoadAscension`
  ;[1 1 1] Load Ascension
  (bind _returnvalue (`GameplayStatics.DoesSaveGameExist` "AscensionSlot"))
  (if _returnvalue
    (bind _returnvalue_2 (`GameplayStatics.LoadGameFromSlot` "AscensionSlot"))
    (bind _assg_saved_ascension (cast `/Game/Islanders/Core/SaveManager/SG_SavedAscension` _returnvalue_2))
    (else
      ;;[1 1 1] Set options to standar settings from Save Game
      (bind _returnvalue_3 (`GameplayStatics.CreateSaveGameObject` "/Game/Islanders/Core/SaveManager/SG_Settings.SG_Settings_C")))))

(fn `hasSavedAscension`
  (returns (HasSavedAscension :type Boolean))
  (bind _returnvalue (`GameplayStatics.DoesSaveGameExist` "AscensionSlot"))
  (if _returnvalue
    (return true)
    (else
      (return false))))

(fn `LoadPlayerStats`
  (returns (HighestAscensionReached :type Integer))
  (bind _returnvalue (`GameplayStatics.DoesSaveGameExist` "PlayerStatSlot"))
  (if _returnvalue
    (bind _returnvalue_2 (`GameplayStatics.LoadGameFromSlot` "PlayerStatSlot"))
    (bind _assg_player_stats (cast `/Game/Islanders/Core/SaveManager/SG_PlayerStats` _returnvalue_2))
    (return (`/Game/Islanders/Core/SaveManager/SG_PlayerStats.HighestAscensionReached` _assg_player_stats))
    (else
      (bind _returnvalue_3 (`GameplayStatics.CreateSaveGameObject` "/Game/Islanders/Core/SaveManager/SG_PlayerStats.SG_PlayerStats_C"))
      (return (`/Game/Islanders/Core/SaveManager/SG_PlayerStats.HighestAscensionReached` _returnvalue_3)))))

(fn `LoadSavedAscension`
  (returns (SavedAscension :type "MySavedAscensionData Structure") (isSavedAscension :type Boolean))
  (bind _returnvalue (`GameplayStatics.DoesSaveGameExist` "AscensionSlot"))
  (if _returnvalue
    (bind _returnvalue_2 (`GameplayStatics.LoadGameFromSlot` "AscensionSlot"))
    (bind _assg_saved_ascension (cast `/Game/Islanders/Core/SaveManager/SG_SavedAscension` _returnvalue_2))
    (return (`/Game/Islanders/Core/SaveManager/SG_SavedAscension.SavedAscension` _assg_saved_ascension) true)
    (else
      (bind _returnvalue_3 (`GameplayStatics.CreateSaveGameObject` "/Game/Islanders/Core/SaveManager/SG_SavedAscension.SG_SavedAscension_C"))
      (return (`/Game/Islanders/Core/SaveManager/SG_SavedAscension.SavedAscension` _returnvalue_3) false))))

(fn `LoadSettings`
  (returns (Settings :type "/Game/Islanders/StartMenu/S_Settings Structure"))
  (bind _returnvalue (`GameplayStatics.DoesSaveGameExist` "SettingSlot"))
  (if _returnvalue
    (bind _returnvalue_2 (`GameplayStatics.LoadGameFromSlot` "SettingSlot"))
    (bind _assg_settings (cast `/Game/Islanders/Core/SaveManager/SG_Settings` _returnvalue_2))
    (return (`/Game/Islanders/Core/SaveManager/SG_Settings.SavedSettingData` _assg_settings))
    (else
      (bind _returnvalue_3 (`GameplayStatics.CreateSaveGameObject` "/Game/Islanders/Core/SaveManager/SG_Settings.SG_Settings_C"))
      (return (`/Game/Islanders/Core/SaveManager/SG_Settings.SavedSettingData` _returnvalue_3)))))

(fn `OnIsNewAscensionReady`
  (returns (isNewAscensionReady :type Boolean))
  (bind _returnvalue (`GameplayStatics.DoesSaveGameExist` "AscensionSlot"))
  (if _returnvalue
    (bind _returnvalue_2 (`GameplayStatics.LoadGameFromSlot` "AscensionSlot"))
    (bind _assg_saved_ascension (cast `/Game/Islanders/Core/SaveManager/SG_SavedAscension` _returnvalue_2))
    (return (`/Game/Islanders/Core/SaveManager/SG_SavedAscension.NewAscensionReady` _assg_saved_ascension))
    (else
      (bind _returnvalue_3 (`GameplayStatics.CreateSaveGameObject` "/Game/Islanders/Core/SaveManager/SG_SavedAscension.SG_SavedAscension_C"))
      (return (`/Game/Islanders/Core/SaveManager/SG_SavedAscension.NewAscensionReady` _returnvalue_3)))))

(fn `OnLoadProgression`
  (returns (Success :type Boolean) (CurrentModifiers :type "Map of String to MyModifierData Structure") (Round :type Integer) (PreviusAscensions :type "Array of /Game/Islanders/Ascension/S_NewAScension Structure"))
  (bind _returnvalue (`GameplayStatics.DoesSaveGameExist` "AscensionSlot"))
  (if _returnvalue
    (bind _returnvalue_2 (`GameplayStatics.LoadGameFromSlot` "AscensionSlot"))
    (bind _assg_saved_ascension (cast `/Game/Islanders/Core/SaveManager/SG_SavedAscension` _returnvalue_2))
    (bind ((`currentModifiers` _currentmodifiers) (`currentRound` _currentround)) (break `MySavedAscensionData` (`/Game/Islanders/Core/SaveManager/SG_SavedAscension.SavedAscension` _assg_saved_ascension)))
    (return true _currentmodifiers _currentround (`/Game/Islanders/Core/SaveManager/SG_SavedAscension.PreviusAscensions` _assg_saved_ascension))
    (else
      (bind _returnvalue_3 (`GameplayStatics.CreateSaveGameObject` "/Game/Islanders/Core/SaveManager/SG_SavedAscension.SG_SavedAscension_C"))
      (bind ((`currentModifiers` _currentmodifiers_2) (`currentRound` _currentround_2)) (break `MySavedAscensionData` (`/Game/Islanders/Core/SaveManager/SG_SavedAscension.SavedAscension` _returnvalue_3)))
      (return false _currentmodifiers_2 _currentround_2 (`/Game/Islanders/Core/SaveManager/SG_SavedAscension.PreviusAscensions` _returnvalue_3)))))

(fn `SaveProgression`
  (params (CurrentModifiers :type "Map of String to MyModifierData Structure") (NewRound :type Integer) (PreviusAscensions :type "Array of /Game/Islanders/Ascension/S_NewAScension Structure"))
  (locals (TempCurrentModifiers :type "Map of String to MyModifierData Structure") (TempNewRound :type Integer) (TempAddCurrentAscension :type "Array of /Game/Islanders/Ascension/S_NewAScension Structure") (NewLocalVar_0 :type String))
  (set `local.TempCurrentModifiers` CurrentModifiers)
  (set `local.TempNewRound` NewRound)
  (set `local.TempAddCurrentAscension` PreviusAscensions)
  (bind _returnvalue (`GameplayStatics.DoesSaveGameExist` "AscensionSlot"))
  (if _returnvalue
    (bind _returnvalue_2 (`GameplayStatics.LoadGameFromSlot` "AscensionSlot"))
    (bind _assg_saved_ascension (cast `/Game/Islanders/Core/SaveManager/SG_SavedAscension` _returnvalue_2))
    (set `/Game/Islanders/Core/SaveManager/SG_SavedAscension.PreviusAscensions` (`local.TempAddCurrentAscension`) _assg_saved_ascension)
    (setmembers `MySavedAscensionData` :`StructRef` (`/Game/Islanders/Core/SaveManager/SG_SavedAscension.SavedAscension` _assg_saved_ascension) :`currentModifiers` (`local.TempCurrentModifiers`) :`currentRound` (`local.TempNewRound`))
    (`GameplayStatics.SaveGameToSlot` _assg_saved_ascension "AscensionSlot")
    (else
      (bind _returnvalue_3 (`GameplayStatics.CreateSaveGameObject` "/Game/Islanders/Core/SaveManager/SG_SavedAscension.SG_SavedAscension_C"))
      (set `/Game/Islanders/Core/SaveManager/SG_SavedAscension.PreviusAscensions` (`local.TempAddCurrentAscension`) _returnvalue_3)
      (setmembers `MySavedAscensionData` :`StructRef` (`/Game/Islanders/Core/SaveManager/SG_SavedAscension.SavedAscension` _returnvalue_3) :`currentModifiers` (`local.TempCurrentModifiers`) :`currentRound` (`local.TempNewRound`))
      (`GameplayStatics.SaveGameToSlot` _returnvalue_3 "AscensionSlot"))))

(fn `TrySavePlayerAscensionRecord`
  (params (CurrentCompletedAscensionLevel :type Integer))
  (locals (TempCompletedAscensionLevel :type Integer))
  (set `local.TempCompletedAscensionLevel` CurrentCompletedAscensionLevel)
  (bind _returnvalue (`GameplayStatics.DoesSaveGameExist` "PlayerStatSlot"))
  (if _returnvalue
    (bind _returnvalue_2 (`GameplayStatics.LoadGameFromSlot` "PlayerStatSlot"))
    (bind _assg_player_stats (cast `/Game/Islanders/Core/SaveManager/SG_PlayerStats` _returnvalue_2))
    (if (> (`local.TempCompletedAscensionLevel`) (`/Game/Islanders/Core/SaveManager/SG_PlayerStats.HighestAscensionReached` _assg_player_stats))
      (`GameplayStatics.SaveGameToSlot` _assg_player_stats "PlayerStatSlot"))
    (else
      (bind _returnvalue_3 (`GameplayStatics.CreateSaveGameObject` "/Game/Islanders/Core/SaveManager/SG_PlayerStats.SG_PlayerStats_C"))
      (set `/Game/Islanders/Core/SaveManager/SG_PlayerStats.HighestAscensionReached` (`local.TempCompletedAscensionLevel`) _returnvalue_3)
      (`GameplayStatics.SaveGameToSlot` _returnvalue_3 "PlayerStatSlot"))))

(fn `UserConstructionScript`)